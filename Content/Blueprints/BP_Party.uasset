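; BP_Party manages a six-slot character party and its on-screen widget.
; On BeginPlay it creates the characters widget, adds the player character to the party and shows the widget on screen.
; Adding rejects duplicates and full parties, fills the first empty slot and refreshes that slot's widget.
; A health event finds a character's slot and updates its health bar.
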(event Custom|UpdateCharacterHealthBar
  (params (CharacterToUpdate :type S%20Character%20Info%20Structure) (Health :type Float%20%28single-precision%29) (MaxHealth :type Float%20%28single-precision%29))
  ;[1 1 1] Update character health bar
  (bind (_ischaracterfound _index) (CallFunction|FindCharacterSlot (.Character (Utilities|Struct|BreakS_CharacterInfo CharacterToUpdate))))
  (if _ischaracterfound
    (Default|UpdateHealthBar (Utilities|Array|Get(acopy) (Variables|/Game/UI/CharactersWidget.CharactersWidget_C|GetSlotsWidgets (Variables|Default|GetCharactersWidget)) _index) Health MaxHealth)))

(event EventBeginPlay
  (Utilities|Array|Resize (Variables|Default|GetCharacters) 6)
  (bind _returnvalue (UserInterface|CreateWidget "/Game/UI/CharactersWidget.CharactersWidget_C" 0 self))
  (bind _asbp_character_base (Utilities|Casting|CastToBP_CharacterBase (Game|GetPlayerCharacter 0)))
  (bind _output_get (Variables|Default|SetCharactersWidget _returnvalue))
  (CallFunction|AddPlayertoParty _asbp_character_base (Variables|/Game/Blueprints/BP_CharacterBase.BP_CharacterBase_C|GetName _asbp_character_base))
  (UserInterface|Viewport|AddtoPlayerScreen _output_get))

(event Collision|EventActorBeginOverlap
  (params (OtherActor :type Actor%20Object%20Reference)))

(event EventTick
  (params (DeltaSeconds :type Float%20%28single-precision%29)))

(fn ConstructionScript)

(fn AddPlayertoParty
  (params (CharacterReference :type BP%20Character%20Base%20Object%20Reference) (CharacterName :type Name))
  (LocalVariables|SetCharacterToAdd (Utilities|Struct|MakeS_CharacterInfo CharacterReference CharacterName))
  (bind _ischaracterfound (CallFunction|FindCharacterSlot CharacterReference))
  (if _ischaracterfound
    (Development|PrintString "Character is already in party!")
    (return false 0)
    (else
      (bind (_isslotemptyfound _indexofemptyslot) (CallFunction|FindEmptySlot))
      (if _isslotemptyfound
        (bind _output_get (LocalVariables|SetLocalIndexOfEmptySlot _indexofemptyslot))
        (Utilities|Array|SetArrayElem (Variables|Default|GetCharacters) _output_get (LocalVariables|GetCharacterToAdd))
        (Utilities|IsValid (Utilities|Array|Get(acopy) (Variables|/Game/UI/CharactersWidget.CharactersWidget_C|GetSlotsWidgets (Variables|Default|GetCharactersWidget)) (LocalVariables|GetLocalIndexOfEmptySlot))
          (:Is%20Valid
            (Default|UpdateSlot (Utilities|Array|Get(acopy) (Variables|/Game/UI/CharactersWidget.CharactersWidget_C|GetSlotsWidgets (Variables|Default|GetCharactersWidget)) (LocalVariables|GetLocalIndexOfEmptySlot))))
          (:Is%20Not%20Valid
            _))
        (return true (LocalVariables|GetLocalIndexOfEmptySlot))
        (else
          (Development|PrintString "No room for character in party!")
          (return false 0))))))

(fn IsSlotEmpty
  (params (Index :type Integer))
  (return (not (Utilities|IsValid (.character (Utilities|Array|Get(acopy) (Variables|Default|GetCharacters) Index))))))

(fn FindEmptySlot
  (bind (_array_element _array_index) (Utilities|Array|ForEachLoopwithBreak (Variables|Default|GetCharacters) :!label _label)
    (:LoopBody
      (if (not (Utilities|IsValid (.Character (Utilities|Struct|BreakS_CharacterInfo _array_element))))
        (LocalVariables|SetLocalIsEmptySlotFound true)
        (LocalVariables|SetLocalIndexOfEmptySlot _array_index)
        (goto _label Break)))
    (:Completed
      (return (LocalVariables|GetLocalIsEmptySlotFound) (LocalVariables|GetLocalIndexOfEmptySlot)))))

(fn FindCharacterSlot
  (params (CharacterToFind :type BP%20Character%20Base%20Object%20Reference))
  (LocalVariables|SetLocalCharacterToFind CharacterToFind)
  (bind (_array_element _array_index) (Utilities|Array|ForEachLoopwithBreak (Variables|Default|GetCharacters) :!label _label)
    (:LoopBody
      (if (== (.Character (Utilities|Struct|BreakS_CharacterInfo _array_element)) (LocalVariables|GetLocalCharacterToFind))
        (LocalVariables|SetLocalIsCharacterFound true)
        (LocalVariables|SetLocalFoundSlotIndex _array_index)
        (goto _label Break)))
    (:Completed
      (return (LocalVariables|GetLocalIsCharacterFound) (LocalVariables|GetLocalFoundSlotIndex)))))