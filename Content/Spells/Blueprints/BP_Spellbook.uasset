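; BP_Spellbook holds a character's learned and memorized spells for Paladin, Priest or Wizard spellbook types.
; Initialization sizes memorized slots from data tables by character level, with Priest and Wizard sharing one table, and learns default spells from each type's master spellbook.
; Memorize, remove and cast events refresh spellbook slot widgets for the selected character.
; Remove and cast also notify the spellcasting widget.
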(event EventBeginPlay)

(event Collision|EventActorBeginOverlap
  (params (OtherActor :type Actor%20Object%20Reference)))

(event EventTick
  (params (DeltaSeconds :type Float%20%28single-precision%29)))

(event EventOnSpellRemoved
  (params (SpellToRemove :type Quest%20Gameplay%20Ability%20Class%20Reference) (SpellLevel :type Integer) (IndexOfRemovedSpell :type Integer))
  (CallFunction|UpdateMemorizedSpellSlotatLevel IndexOfRemovedSpell SpellLevel))

(event EventOnSpellCast
  (params (DisabledSpell :type Quest%20Gameplay%20Ability%20Class%20Reference) (SpellLevel :type Integer) (IndexOfDisabledSpell :type Integer))
  (CallFunction|UpdateMemorizedSpellSlotatLevel IndexOfDisabledSpell SpellLevel))

(event EventOnSpellMemorized
  (params (Level :type Integer) (SpellSlot :type Integer))
  (CallFunction|UpdateMemorizedSpellSlotonCurrentLevel SpellSlot))

(fn ConstructionScript)

(fn SetNumberOfMemorizedSpellsPerLevel
  (bind _numberofmemorizedspellsbylevel (Variables|Default|GetNumberOfMemorizedSpellsByLevel))
  (bind _numberofmemorizedspellsbylevel_2 (Variables|Default|GetNumberOfMemorizedSpellsByLevel))
  (bind _numberofmemorizedspellsbylevel_3 (Variables|Default|GetNumberOfMemorizedSpellsByLevel))
  (bind _numberofmemorizedspellsbylevel_4 (Variables|Default|GetNumberOfMemorizedSpellsByLevel))
  (bind _numberofmemorizedspellsbylevel_5 (Variables|Default|GetNumberOfMemorizedSpellsByLevel))
  (LocalVariables|SetLocalRowName (Utilities|String|StringToName (Utilities|String|ToString(Integer) (Math|Float|Truncate (.currentvalue (Variables|/Script/Quest.QuestAttributeSet|GetLevel (Variables|/Script/Quest.QuestCharacterBase|GetAttributeSetComponent (Variables|Default|GetOwningCharacter))))))))
  (switch Utilities|FlowControl|Switch|SwitchonESpellType (Variables|Default|GetSpellbookType)
    (:IT_Paladin
      (bind _returnvalue (Utilities|GetDataTableRow "/Game/Spells/Blueprints/DataTables/PaladinSpellSlotTable.PaladinSpellSlotTable" (LocalVariables|GetLocalRowName))
        (:then
          (Utilities|Array|Clear _numberofmemorizedspellsbylevel_5)
          (Utilities|Array|Resize _numberofmemorizedspellsbylevel_5 5)
          (Utilities|Array|SetArrayElem _numberofmemorizedspellsbylevel_5 0 (.level1slots _returnvalue))
          (Utilities|Array|SetArrayElem _numberofmemorizedspellsbylevel 1 (.level2slots _returnvalue))
          (Utilities|Array|SetArrayElem _numberofmemorizedspellsbylevel 2 (.level3slots _returnvalue))
          (Utilities|Array|SetArrayElem _numberofmemorizedspellsbylevel 3 (.level4slots _returnvalue))
          (Utilities|Array|SetArrayElem _numberofmemorizedspellsbylevel 4 (.level5slots _returnvalue))
          (return))
        (:RowNotFound
          _)))
    (:IT_Priest
      (bind _returnvalue_2 (Utilities|GetDataTableRow "/Game/Spells/Blueprints/DataTables/SpellSlotsTable.SpellSlotsTable" (LocalVariables|GetLocalRowName) :!label _label)
        (:then
          (Utilities|Array|Clear _numberofmemorizedspellsbylevel_3)
          (Utilities|Array|Resize _numberofmemorizedspellsbylevel_3 9)
          (Utilities|Array|SetArrayElem _numberofmemorizedspellsbylevel_3 0 (.level1slots _returnvalue_2))
          (Utilities|Array|SetArrayElem _numberofmemorizedspellsbylevel_2 1 (.level2slots _returnvalue_2))
          (Utilities|Array|SetArrayElem _numberofmemorizedspellsbylevel_2 2 (.level3slots _returnvalue_2))
          (Utilities|Array|SetArrayElem _numberofmemorizedspellsbylevel_2 3 (.level4slots _returnvalue_2))
          (Utilities|Array|SetArrayElem _numberofmemorizedspellsbylevel_2 4 (.level5slots _returnvalue_2))
          (Utilities|Array|SetArrayElem _numberofmemorizedspellsbylevel_4 5 (.level6slots _returnvalue_2))
          (Utilities|Array|SetArrayElem _numberofmemorizedspellsbylevel_4 6 (.level7slots _returnvalue_2))
          (Utilities|Array|SetArrayElem _numberofmemorizedspellsbylevel_4 7 (.level8slots _returnvalue_2))
          (Utilities|Array|SetArrayElem _numberofmemorizedspellsbylevel_4 8 (.level9slots _returnvalue_2))
          (return))
        (:RowNotFound
          _)))
    (:IT_Wizard
      (goto _label))
    (:IT_Other
      (return)))
  (return))

(fn InitializeMemorizedArrays
  (CallFunction|SetNumberOfMemorizedSpellsPerLevel)
  (Class|QuestSpellbook|SetMemorizedArraySizes)
  (return))

(fn InitializeLearnedSpellArrays
  (Class|QuestSpellbook|SetSizeOfLearnedSpells)
  (for (_ _array_index) (Variables|Default|GetLearnedSpells)
    (CallFunction|LearnDefaultSpellsatLevel _array_index))
  (return))

(fn InitializeArrays
  (CallFunction|SetNumberOfMemorizedSpellsPerLevel)
  (CallFunction|InitializeLearnedSpellArrays)
  (CallFunction|InitializeMemorizedArrays)
  (return))

(fn LearnDefaultSpellsatLevel
  (params (SpellLevelIndex :type Integer))
  (LocalVariables|SetLocalSpellLevel SpellLevelIndex)
  (switch Utilities|FlowControl|Switch|SwitchonESpellType (Variables|Default|GetSpellbookType)
    (:IT_Paladin
      (LocalVariables|SetSpellsAtLevel (Variables|/Script/Quest.QuestSpells|GetSpells (Utilities|Array|Get(acopy) (Variables|Default|GetMasterPaladinSpellbook) (LocalVariables|GetLocalSpellLevel)))))
    (:IT_Priest
      (LocalVariables|SetSpellsAtLevel (Variables|/Script/Quest.QuestSpells|GetSpells (Utilities|Array|Get(acopy) (Variables|Default|GetMasterPriestSpellbook) (LocalVariables|GetLocalSpellLevel)))))
    (:IT_Wizard
      (LocalVariables|SetSpellsAtLevel (Variables|/Script/Quest.QuestSpells|GetSpells (Utilities|Array|Get(acopy) (Variables|Default|GetMasterWizardSpellbook) (LocalVariables|GetLocalSpellLevel)))))
    (:IT_Other
      (return)))
  (for _array_element (LocalVariables|GetSpellsAtLevel)
    (if (.bisdefaultspell _array_element)
      (Class|QuestSpellbook|LearnSpell (.spell _array_element))))
  (return))

(fn UpdateMemorizedSpellSlotonCurrentLevel
  (params (SpellIndex :type Integer))
  (LocalVariables|SetLocalSpellIndex SpellIndex)
  (bind _asbp_character_base (Utilities|Casting|CastToBP_CharacterBase (Variables|Default|GetOwningCharacter))
    (:then
      (if (== _asbp_character_base (Variables|/Script/Quest.QuestPlayerController|GetSelectedCharacter (Variables|/Game/Inventory/Blueprints/BP_Inventory.BP_Inventory_C|GetOwningController (Variables|/Game/Blueprints/BP_CharacterBase.BP_CharacterBase_C|GetInventory _asbp_character_base))))
        (Default|UpdateSlot (Utilities|Array|Get(acopy) (Variables|/Game/Spells/Widgets/SpellbookWidget.SpellbookWidget_C|GetMemorizedSpellsSlotWidgets (Variables|/Game/Blueprints/BP_PlayerController.BP_PlayerController_C|GetSpellbookWidget (Variables|/Game/Inventory/Blueprints/BP_Inventory.BP_Inventory_C|GetOwningController (Variables|/Game/Blueprints/BP_CharacterBase.BP_CharacterBase_C|GetInventory _asbp_character_base)))) (LocalVariables|GetLocalSpellIndex)))
        (return)
        (else
          (return))))
    (:CastFailed
      (return))))

(fn UpdateMemorizedSpellSlotatLevel
  (params (SpellIndex :type Integer) (SpellLevel :type Integer))
  ;[1 1 1] Set local variables
  (LocalVariables|SetLocalSpellIndex SpellIndex)
  (LocalVariables|SetLocalSpellLevel SpellLevel)
  ;[1 1 1] Verify that the player is in the party by checking whether it has an inventory reference
  (bind _asbp_character_base (Utilities|Casting|CastToBP_CharacterBase (Variables|Default|GetOwningCharacter))
    (:then
      (bind _owningcontroller (Variables|/Game/Inventory/Blueprints/BP_Inventory.BP_Inventory_C|GetOwningController (Variables|/Game/Blueprints/BP_CharacterBase.BP_CharacterBase_C|GetInventory _asbp_character_base))
        (:then
          ;[1 1 1] If the right spellbook is open to the appropriate level, update it
          (LocalVariables|SetLocalPlayerController _owningcontroller)
          (if (== _asbp_character_base (Variables|/Script/Quest.QuestPlayerController|GetSelectedCharacter _owningcontroller))
            (if (== (LocalVariables|GetLocalSpellLevel) (Variables|/Game/Spells/Widgets/SpellbookWidget.SpellbookWidget_C|GetActiveSpellLevel (Variables|/Game/Blueprints/BP_PlayerController.BP_PlayerController_C|GetSpellbookWidget (LocalVariables|GetLocalPlayerController))))
              ;;[0 0.07082 1] Update the spellbook's memorized slot
              (Default|UpdateSlot (Utilities|Array|Get(acopy) (Variables|/Game/Spells/Widgets/SpellbookWidget.SpellbookWidget_C|GetMemorizedSpellsSlotWidgets (Variables|/Game/Blueprints/BP_PlayerController.BP_PlayerController_C|GetSpellbookWidget (LocalVariables|GetLocalPlayerController))) (LocalVariables|GetLocalSpellIndex)))))
          ;[1 1 1] Update spell casting widget if it's on the right page
          (Default|CheckifSpellsShouldbeUpdated (Variables|/Game/Blueprints/BP_PlayerController.BP_PlayerController_C|GetSpellcastingWidget (LocalVariables|GetLocalPlayerController)) self (LocalVariables|GetLocalSpellLevel))
          (return))
        (:else
          (return))))
    (:CastFailed
      (return))))