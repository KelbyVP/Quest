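; Base Gameplay Ability for player and party spells, providing shared setup and completion handling.
; On activation it caches the quest character, reads the order target and location from its AI Blackboard, and picks the projectile casting montage.
; An overridable step then adjusts range by character level.
; Success and abort events notify the character that casting finished, removing the spell from memorized spells only on success.
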(event Custom|OnSuccessfulCast
  ;[1 1 1] On successful cast
  (Class|QuestCharacterBase|OnFinishedCastingSpell (Variables|Default|GetCharacter) (Utilities|GetClass self) true))

(event Custom|OnAbortedCast
  ;[1 1 1] On aborted cast
  (Class|QuestCharacterBase|OnFinishedCastingSpell (Variables|Default|GetCharacter) (Utilities|GetClass self) false))

(event Ability|EventActivateAbility
  ;[1 1 1] Activate ability
  (CallFunction|SetCharacterVariables)
  ;;[0 0.07082 1] Simple range adjustment; override for custom range adjustments
  (CallFunction|AdjustRange))

(fn GetCharacterandPlayerControllerInfo
  (bind _asquest_character_base (Utilities|Casting|CastToQuestCharacterBase (Ability|GetOwningActorfromActorInfo))
    (:then
      (bind _asbp_player_controller (Utilities|Casting|CastToBP_PlayerController (Game|GetPlayerController 0))
        (:then
          (return _asquest_character_base _asbp_player_controller))
        (:CastFailed
          _)))
    (:CastFailed
      _))
  (CallFunction|OnAbortedCast)
  (Ability|EndAbility))

(fn SetCharacterVariables
  (bind _character (CallFunction|GetCharacterandPlayerControllerInfo))
  (bind _output_get (Variables|Default|SetCharacter _character))
  (bind _asaicontroller (Utilities|Casting|CastToAIController (Pawn|GetController _output_get))
    (:then
      (LocalVariables|SetBlackboard (AI|GetBlackboard _asaicontroller))
      (Variables|Default|SetActorToTarget (AI|Components|Blackboard|GetValueasObject (AI|GetBlackboard _asaicontroller) (Utilities|String|StringToName "Order_Target")))
      (Variables|Default|SetLocationToTarget (AI|Components|Blackboard|GetValueasVector (LocalVariables|GetBlackboard) (Utilities|String|StringToName "Order_Location")))
      (CallFunction|SetSpellcastingMontage)
      (bind _output_get_2 (Variables|Default|SetCharacterLevel (Math|Float|Truncate (.currentvalue (Variables|/Script/Quest.QuestAttributeSet|GetLevel (Variables|/Script/Quest.QuestCharacterBase|GetAttributeSetComponent (Variables|Default|GetCharacter)))))))
      (return _output_get_2))
    (:CastFailed
      (return 0))))

(fn SetSpellcastingMontage
  (bind _returnvalue (Class|QuestCharacterBase|GetProjectileSpellcastingMontage (Variables|Default|GetCharacter)))
  (Variables|Default|SetAnimMontageToPlay _returnvalue)
  (return))

(fn AdjustRange
  (Class|QuestGameplayAbility|AdjustRangebyCharacterLevel (.currentvalue (Variables|/Script/Quest.QuestAttributeSet|GetLevel (Variables|/Script/Quest.QuestCharacterBase|GetAttributeSetComponent (Variables|Default|GetCharacter)))))
  (return))