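; BP_GASpellBase is a Gameplay Ability System base ability for spells, holding setup and cleanup logic.
; On activation it resolves the owning BP_CharacterBase and player controller, then caches the character, its level from the attribute set, and its projectile spell montage.
; On end it notifies the character which spell class finished, flagging it for removal from memorized spells unless the ability was cancelled.
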(event Ability|EventActivateAbility
  (CallFunction|SetCharacterVariables))

(event Ability|EventOnEndAbility
  (params (bWasCancelled :type Boolean))
  (Default|OnSpellFinished (Variables|Default|GetCharacter) (Utilities|GetClass self) (not bWasCancelled)))

(fn GetCharacterandControllerInfo
  (bind _asbp_character_base (Utilities|Casting|CastToBP_CharacterBase (Ability|GetOwningActorfromActorInfo))
    (:then
      (bind _asbp_player_controller (Utilities|Casting|CastToBP_PlayerController (Pawn|GetController _asbp_character_base)))
      (return _asbp_character_base _asbp_player_controller))
    (:CastFailed
      (return 0 0))))

(fn SetCharacterVariables
  (bind _characterbase (CallFunction|GetCharacterandControllerInfo))
  (Variables|Default|SetCharacter _characterbase)
  (bind _output_get (Variables|Default|SetCharacterLevel (Math|Float|Truncate (.currentvalue (Variables|/Script/Quest.QuestAttributeSet|GetLevel (Variables|/Script/Quest.QuestCharacterBase|GetAttributeSetComponent (Variables|Default|GetCharacter)))))))
  (Variables|Default|SetAnimMontageToPlay (Variables|/Game/Blueprints/BP_CharacterBase.BP_CharacterBase_C|GetSpellMontage_Projectile (Variables|Default|GetCharacter)))
  (return _output_get))