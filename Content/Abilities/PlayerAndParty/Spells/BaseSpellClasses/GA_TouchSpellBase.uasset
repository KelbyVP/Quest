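; Base gameplay ability for touch spells that apply a gameplay effect to a single target actor.
; On activation it runs parent setup, aborts without a valid target actor, and otherwise plays the casting montage.
; A tagged gameplay event commits the ability, applies the effect at character level, calls OnSuccessfulCast and ends.
; Any montage finish, blend out, interruption or cancel calls OnAbortedCast and ends the ability.
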(event Ability|EventActivateAbility
  ;[1 1 1] Set variables for ability and verify we have  valid target
  (|CallParentFunction)
  (bind _asactor (Utilities|Casting|CastToActor (Variables|Default|GetActorToTarget))
    (:then
      (Variables|Default|SetTargetData (Ability|TargetData|AbilityTargetDatafromActor _asactor))
      ;[1 1 1] Play spellcasting montage
      (|PlayMontageandWaitProxy "None" (Variables|Default|GetAnimMontageToPlay) 1.0 "None" true 1.0
        (:then
          (Ability|Tasks|WaitGameplayEvent (Variables|Default|GetEventTag) 0
            (:EventReceived
              ;[1 1 1] Execute ability
              (Ability|CommitAbility)
              (GameplayEffects|ApplyGameplayEffectToTarget (Variables|Default|GetTargetData) (Variables|Default|GetGameplayEffectClass) (Variables|Default|GetCharacterLevel) 1)
              (CallFunction|OnSuccessfulCast)
              (Ability|EndAbility))))
        (:OnCompleted
          (CallFunction|OnAbortedCast :!label _label)
          (Ability|EndAbility))
        (:OnBlendOut
          (goto _label))
        (:OnInterrupted
          (goto _label))
        (:OnCancelled
          (goto _label))))
    (:CastFailed
      (CallFunction|OnAbortedCast)
      (Ability|EndAbility))))

(event Ability|EventOnEndAbility
  (params (bWasCancelled :type Boolean))
  (|CallParentFunction bWasCancelled) ; This node is disabled and will not be called.\nDrag off pins to build functionality.
)