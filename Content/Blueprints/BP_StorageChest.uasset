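; Storage chest actor that lets the player open a slot-based item storage alongside their inventory.
; Interacting passes a DoOnce gate, lazily spawns a BP_StorageItems actor with the chest's slot layout, then shows both panels, falling back to player controller 0 if needed.
; Closing, also triggered when the linked QuestCharacter ends overlap, hides both panels and resets the gate.
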(event Custom|OnStorageClosed
  ;[0 0.2708 0.03765] On Storage Closed
  (Utilities|IsValid (Variables|Default|GetStorageItems)
    (:Is%20Valid
      (Default|HideStorage (Variables|Default|GetStorageItems))
      (bind _playercontroller (Variables|Default|GetPlayerController)
        (:then
          (if (Variables|/Game/Inventory/Blueprints/BP_Inventory.BP_Inventory_C|GetIsVisible (Variables|/Game/Blueprints/BP_PlayerController.BP_PlayerController_C|GetInventory _playercontroller))
            (Default|HideInventory (Variables|/Game/Blueprints/BP_PlayerController.BP_PlayerController_C|GetInventory _playercontroller))
            ;[0 0.2708 0.03765] On Interact
            (Utilities|FlowControl|DoOnce false) ; enters at Reset
            (else
              (Utilities|FlowControl|DoOnce false) ; enters at Reset
            )))
        (:else)))))

(event EventBeginPlay)

(event Collision|EventActorEndOverlap
  (params (OtherActor :type Actor%20Object%20Reference))
  (bind _asquest_character (Utilities|Casting|CastToQuestCharacter OtherActor))
  (if (== self (Variables|/Script/Quest.QuestCharacter|GetStorageChest _asquest_character))
    (Variables|/Script/Quest.QuestCharacter|SetStorageChest _asquest_character 0)
    (CallFunction|OnStorageClosed)))

(event EventTick
  (params (DeltaSeconds :type Float%20%28single-precision%29)))

(event EventOnInteract
  (params (PlayerController :type Quest%20Player%20Controller%20Object%20Reference))
  ;[0 0.2708 0.03765] On Interact
  (Utilities|FlowControl|DoOnce false
    (:Completed
      (bind _asbp_player_controller (Utilities|Casting|CastToBP_PlayerController PlayerController)
        (:then
          (Variables|Default|SetPlayerController _asbp_player_controller))
        (:CastFailed
          (bind _asbp_player_controller_2 (Utilities|Casting|CastToBP_PlayerController (Game|GetPlayerController 0)))
          (Variables|Default|SetPlayerController _asbp_player_controller_2)))
      (Utilities|IsValid (Variables|Default|GetStorageItems)
        (:Is%20Valid
          _)
        (:Is%20Not%20Valid
          (bind _returnvalue (Game|SpawnActorfromClass "/Game/Inventory/Blueprints/BP_StorageItems.BP_StorageItems_C" (Math|Transform|MakeTransform "0, 0, 0" "0, 0, 0" "1,1,1") "AlwaysSpawn" 0 (Variables|Default|GetAmountOfSlots) (Variables|Default|GetPlayerController) 0 (Variables|Default|GetSlotsPerRow) self 0))
          (bind _output_get (Variables|Default|SetStorageItems _returnvalue))))
      (Default|GenerateSlotWidgets (Variables|/Game/Inventory/Blueprints/BP_StorageItems.BP_StorageItems_C|GetStorageWidget (Variables|Default|GetStorageItems)) _output_get)
      (Default|ShowStorage (Variables|Default|GetStorageItems))
      (Default|HideInventory (Variables|/Game/Blueprints/BP_PlayerController.BP_PlayerController_C|GetInventory (Variables|Default|GetPlayerController)))
      (Default|ShowInventory (Variables|/Game/Blueprints/BP_PlayerController.BP_PlayerController_C|GetInventory (Variables|Default|GetPlayerController))))))

(fn ConstructionScript)