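; Base gameplay ability for spells that affect every actor within range of the caster, with target filtering left for child spells to override.
; On launch, an instant target data task gathers actors around the character's location using the spell's range, then applies the gameplay effect to them.
; A cancelled search or empty result aborts and ends the ability.
; A gameplay cue plays casting effects before the cast.
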(event Ability|EventActivateAbility
  (|CallParentFunction) ; This node is disabled and will not be called.\nDrag off pins to build functionality.
)

(event Ability|EventOnEndAbility
  (params (bWasCancelled :type Boolean))
  (|CallParentFunction bWasCancelled) ; This node is disabled and will not be called.\nDrag off pins to build functionality.
)

(event EventLaunchPostCastingEffects)

(event EventOnProjectileLaunched
  ;[1 1 1] Get actors in range
  (bind _data (|WaitTargetData :ConfirmationType "Instant" :Class "/Script/Quest.QuestGATargetActorsInRange" :TargetLocation (Transformation|GetActorLocation (Variables|Default|GetCharacter)) :TargetRadius (Variables|Default|GetRange))
    (:then
      (Variables|Default|SetTargetData _data)
      (CallFunction|ApplyEffectstoTargets))
    (:Cancelled
      (CallFunction|OnAbortedCast)
      (Ability|EndAbility))))

(event EventLaunchPreCastingEffects
  (CallFunction|LaunchCastingEffectsDuringCasting))

(fn ApplyEffectstoTargets
  ;[1 1 1] Verify we have at least one target character
  (if (Ability|TargetData|TargetDataHasActor (Variables|Default|GetTargetData))
    ;[1 1 1] Filter targets:  Override this function to ensure effects apply only to appropriate actors in range
    (CallFunction|FilterTargets)
    ;[1 1 1] Apply effect to characters in range
    (GameplayEffects|ApplyGameplayEffectToTarget (Variables|Default|GetTargetData) (Variables|Default|GetGameplayEffectClass) 1 1)
    (else
      (Class|QuestOrderHelperLibrary|AbortOrder)
      (Ability|EndAbility))))

(fn FilterTargets
  (return))

(fn LaunchCastingEffectsDuringCasting
  (GameplayCue|ExecuteGameplayCue :GameplayCueTag (Variables|Default|GetCastingEffectsTag))
  (return))