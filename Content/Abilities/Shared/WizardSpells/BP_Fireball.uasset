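; BP_Fireball is the wizard fireball spell projectile, which flies to a target location and explodes.
; On BeginPlay it scales itself by caster level, then a timeline lerps it to a point just above the target without sweeping.
; On arrival it spawns a level-scaled explosion, applies the ability-supplied GameplayEffect spec to QuestCharacterBase actors from the supplied target data, and destroys itself.
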(event EventBeginPlay
  (bind _level (Variables|Default|GetLevel))
  (bind _level_2 (Variables|Default|GetLevel))
  (bind _returnvalue (- _level 2))
  (bind _returnvalue_2 (- _level_2 1))
  (bind _returnvalue_3 (/ _returnvalue 3))
  (bind _returnvalue_4 (/ _returnvalue_2 3))
  (bind _returnvalue_5 (Math|Integer|Clamp(Integer) _returnvalue_3 1 6))
  (bind _returnvalue_6 (Math|Integer|Clamp(Integer) _returnvalue_4 1 6))
  (bind _returnvalue_7 (Math|Conversions|ToFloat(Integer) _returnvalue_5))
  (bind _returnvalue_8 (Math|Conversions|ToFloat(Integer) _returnvalue_6))
  ;[1 1 1] Scale size of fireball based on character's level
  (Transformation|SetActorScale3D (Math|Vector|MakeVector _returnvalue_8 _returnvalue_8 _returnvalue_8))
  ;[1 1 1] Set start and target locations
  (Variables|Default|SetStartLocation (Transformation|GetActorLocation))
  (Variables|Default|SetTargetLocation (Math|Vector|MakeVector (.x (Variables|Default|GetTargetLocation)) (.y (Variables|Default|GetTargetLocation)) (+ (.z (Variables|Default|GetTargetLocation)) 1e+02)))
  ;[1 1 1] Move fireball to target location
  (bind _location (Timeline|Timeline_0_0 Play)
    (:Update
      (Transformation|SetActorLocation (Math|Vector|Lerp(Vector) (Variables|Default|GetStartLocation) (Variables|Default|GetTargetLocation) _location) false false))
    (:Finished
      ;[1 1 1] Spawn explosion
      (Effects|SpawnEmitteratLocation "/Game/Effects/FXVarietyPack/Particles/P_ky_explosion.P_ky_explosion" (Variables|Default|GetTargetLocation) "0, 0, 0" (Math|Vector|MakeVector _returnvalue_7 _returnvalue_7 _returnvalue_7))
      (CallFunction|DamageActorsinRange)
      (Actor|DestroyActor))))

(event Collision|EventActorBeginOverlap
  (params (OtherActor :type Actor%20Object%20Reference)))

(event EventTick
  (params (DeltaSeconds :type Float%20%28single-precision%29)))

(fn ConstructionScript)

(fn DamageActorsinRange
  (for _array_element (Ability|TargetData|GetActorsfromTargetData (Variables|Default|GetGADataHandleStruct))
    (Utilities|Casting|CastToQuestCharacterBase _array_element)
    (Class|QuestFunctionLibrary|ApplyGameplayEffectSpecHandletoTargetDataHandleSpecHandle (Variables|Default|GetEffectSpecHandleFromAbility) (Ability|TargetData|AbilityTargetDatafromActor _array_element)))
  (return))