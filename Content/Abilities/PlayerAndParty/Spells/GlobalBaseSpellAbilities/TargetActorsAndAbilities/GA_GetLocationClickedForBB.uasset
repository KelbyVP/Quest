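; Helper gameplay ability that lets the player pick a ground location for a spell order and stores it on the character controller's Blackboard.
; It reads the ground-target spell class from Order_Ability and uses that class's default radius for a WaitTargetData decal targeting actor.
; On confirmation it writes the clicked point to Order_Location and ends.
; On cancel it calls OnAbortedCast before ending.
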(event Ability|EventActivateAbility
  (|CallParentFunction)
  ;[1 1 1] Get targeting data
  (bind _asga_ground_target_ability_spell_base (Utilities|Casting|CastToGA_GroundTargetAbilitySpellBaseClass (Class|BlackboardComponent|GetValueasClass (AI|GetBlackboard (Pawn|GetController (Variables|Default|GetCharacter))) (Utilities|String|StringToName "Order_Ability"))))
  (bind _data (|WaitTargetData :ConfirmationType "UserConfirmed" :Class "/Game/Abilities/PlayerAndParty/Spells/GlobalBaseSpellAbilities/TargetActorsAndAbilities/BP_GroundTargetSelectActor.BP_GroundTargetSelectActor_C" :DecalMaterial "/Game/Materials/Decals/M_FireballDecal.M_FireballDecal" :TestDecal "/Game/Materials/Decals/M_FireballDecal.M_FireballDecal" :Radius (.Radius (Utilities|GetClassDefaults _asga_ground_target_ability_spell_base)) :ReticleClass 0)
    (:ValidData
      (Variables|Default|SetTargetData _data)
      ;[1 1 1] Get the location we clicked on
      (Variables|Default|SetLocation (Class|AbilitySystemBlueprintLibrary|GetTargetDataEndPoint (Variables|Default|GetTargetData) (- (Ability|TargetData|GetDataCountfromTargetData (Variables|Default|GetTargetData)) 1)))
      ;[1 1 1] Set blackboard value as target selected
      (AI|Components|Blackboard|SetValueasVector (AI|GetBlackboard (Pawn|GetController (Variables|Default|GetCharacter))) (Utilities|String|StringToName "Order_Location") (Variables|Default|GetLocation))
      (Ability|EndAbility))
    (:Cancelled
      (CallFunction|OnAbortedCast)
      (Ability|EndAbility))))

(event Ability|EventOnEndAbility
  (params (bWasCancelled :type Boolean)))