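; BP_QuestBase is a base quest Blueprint that connects quest logic to the player's inventory and the journal UI.
; It checks for required items by querying the player controller's inventory through the QuestManager.
; On goal completion, goals flagged for it append their update text to the current description.
; If the quest is selected in the journal, the journal description refreshes through BP_QuestManager's main widget.
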(fn ConstructionScript)

(fn BPHasInventoryItem
  (params (Item :type Quest%20Item%20Object%20Reference))
  (bind _output_get (LocalVariables|SetLocalItem Item))
  (Utilities|IsValid _output_get
    (:Is%20Valid
      (bind _asbp_player_controller (Utilities|Casting|CastToBP_PlayerController (Variables|/Script/Quest.QuestQuestManager|GetPlayerController (Variables|Default|GetQuestManager)))
        (:then
          (bind _isininventory (Default|FindIteminInventory (Variables|/Game/Blueprints/BP_PlayerController.BP_PlayerController_C|GetInventory _asbp_player_controller) (LocalVariables|GetLocalItem)))
          (return _isininventory))
        (:CastFailed
          (return false))))
    (:Is%20Not%20Valid
      (return false))))

(fn BPonGoalCompleted
  (params (GoalIndex :type Integer))
  (bind _returnvalue (Class|QuestQuestBase|GetGoalatIndex GoalIndex))
  ;[1 1 1] Update quest description
  (if (.ShouldUpdateQuestDescriptionUponCompletion (Utilities|Struct|BreakGoalData _returnvalue))
    (Variables|Default|SetCurrentDescription (Utilities|Text|FormatText "{Current}|{Update}" (Variables|Default|GetCurrentDescription) (.UpdatedQuestDescription (Utilities|Struct|BreakGoalData _returnvalue))))
    (if (CallFunction|IsSelectedinJournal)
      (bind _asbp_quest_manager (Utilities|Casting|CastToBP_QuestManager (Variables|Default|GetQuestManager))
        (:then
          (Default|UpdateDescription (Variables|/Game/UI/MainWidget.MainWidget_C|GetJournal (Variables|/Game/Quests/Blueprints/BP_QuestManager.BP_QuestManager_C|GetMainWidget _asbp_quest_manager))))
        (:CastFailed
          _))
      (return)
      (else
        (return)))
    (else
      (return))))

(fn IsSelectedinJournal
  (bind _asbp_quest_manager (Utilities|Casting|CastToBP_QuestManager (Variables|Default|GetQuestManager))
    (:then
      (return (and (Utilities|IsValid (Variables|/Game/Quests/Widgets/Journal.Journal_C|GetSelectedQuest (Variables|/Game/UI/MainWidget.MainWidget_C|GetJournal (Variables|/Game/Quests/Blueprints/BP_QuestManager.BP_QuestManager_C|GetMainWidget _asbp_quest_manager)))) (== (Variables|/Game/Quests/Widgets/Journal.Journal_C|GetSelectedQuest (Variables|/Game/UI/MainWidget.MainWidget_C|GetJournal (Variables|/Game/Quests/Blueprints/BP_QuestManager.BP_QuestManager_C|GetMainWidget _asbp_quest_manager))) self))))
    (:CastFailed
      (return false))))