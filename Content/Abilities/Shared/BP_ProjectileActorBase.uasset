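; Base projectile actor for abilities that travels to a target location and applies a gameplay effect on arrival.
; On BeginPlay, a timeline lerps it from its spawn point to TargetLocation without sweep or overlap checks.
; When the timeline finishes, DamageTargets applies the ability-supplied effect spec to each actor in the stored GAS target data (index 0).
; The actor then destroys itself.
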(event EventBeginPlay
  (Variables|Default|SetStartLocation (Transformation|GetActorLocation))
  (bind _projectilemovementtimeline (Timeline|Timeline_0 Play)
    (:Update
      (Transformation|SetActorLocation (Math|Vector|Lerp(Vector) (Variables|Default|GetStartLocation) (Variables|Default|GetTargetLocation) _projectilemovementtimeline) false false))
    (:Finished
      (CallFunction|DamageTargets)
      (Actor|DestroyActor))))

(event Collision|EventActorBeginOverlap
  (params (OtherActor :type Actor%20Object%20Reference)))

(event EventTick
  (params (DeltaSeconds :type Float%20%28single-precision%29)))

(fn ConstructionScript)

(fn DamageTargets
  (for _array_element (Ability|TargetData|GetActorsfromTargetData (Variables|Default|GetGADataHandleStruct))
    (Class|QuestFunctionLibrary|ApplyGameplayEffectSpecHandletoTargetDataHandleSpecHandle (Variables|Default|GetEffectSpecHandleFromAbility) (Ability|TargetData|AbilityTargetDatafromActor _array_element)))
  (return))