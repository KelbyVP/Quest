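; Priest Light Healing gameplay ability that applies a gameplay effect to a clicked, non-hostile character.
; It waits for user-confirmed actor targeting, rejecting cancelled, non-character or hostile picks as aborted casts.
; A valid pick plays a cast montage; a gameplay event then commits the ability and applies the effect at character level.
; Montage completion, blend-out, interruption or cancellation aborts the cast and ends the ability.
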(event Ability|EventActivateAbility
  (|CallParentFunction)
  ;[1 1 1] Get targeting data
  (bind _data (|WaitTargetData :ConfirmationType "UserConfirmed" :Class "/Script/Quest.QuestGATargetActorClicked")
    (:ValidData
      (bind _output_get (Variables|Default|SetTargetData _data))
      ;[1 1 1] Verify we clicked on a character
      (if (Ability|TargetData|TargetDataHasActor _output_get)
        ;[1 1 1] Verify the target is not hostile
        (bind _asquest_character_base (Utilities|Casting|CastToQuestCharacterBase (Utilities|Array|Get(acopy) (Ability|TargetData|GetActorsfromTargetData (Variables|Default|GetTargetData))))
          (:then
            (Variables|Default|SetTargetCharacter _asquest_character_base)
            (if (Variables|/Script/Quest.QuestCharacterBase|GetbIsHostile _asquest_character_base)
              (CallFunction|OnAbortedCast :!label _label)
              (Ability|EndAbility)
              (else
                (|PlayMontageandWaitProxy "None" (Variables|Default|GetAnimMontageToPlay) 1.0 "None" true 1.0
                  (:then
                    (Ability|Tasks|WaitGameplayEvent (Variables|Default|GetEventTagToTriggerHealing) 0
                      (:EventReceived
                        (Ability|CommitAbility)
                        (GameplayEffects|ApplyGameplayEffectToTarget (Variables|Default|GetTargetData) (Variables|Default|GetGameplayEffectClass) (Variables|Default|GetCharacterLevel) 1)
                        (CallFunction|OnSuccessfulCast)
                        (Ability|EndAbility))))
                  (:OnCompleted
                    (CallFunction|OnAbortedCast :!label _label_2)
                    (Ability|EndAbility))
                  (:OnBlendOut
                    (goto _label_2))
                  (:OnInterrupted
                    (goto _label_2))
                  (:OnCancelled
                    (goto _label_2))))))
          (:CastFailed
            (goto _label)))
        (else
          (CallFunction|OnAbortedCast)
          (Ability|EndAbility))))
    (:Cancelled
      (CallFunction|OnAbortedCast)
      (Ability|EndAbility))))

(event Ability|EventOnEndAbility
  (params (bWasCancelled :type Boolean))
  (|CallParentFunction bWasCancelled) ; This node is disabled and will not be called.\nDrag off pins to build functionality.
)