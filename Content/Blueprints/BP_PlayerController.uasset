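; Player controller for a party-based RPG, handling character selection, UI panels, ability hotkeys and pause.
; BeginPlay spawns the inventory, party and off-world 3D mesh capture actor, then links the spellbook and spellcasting widgets.
; Selection changes refresh equipment, mesh preview and spell widgets, while opening the spellbook closes competing panels.
; Hotkeys activate GAS abilities on the selected character, add or rest party members, and pause through zero global time dilation.
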(event Custom|UpdateGold_1
  ;[0 0.01307 1] Inventory functionality
  ;;[1 1 1] Update gold
)

(event EventBeginPlay
  ;[0.001565 0 0.5052] Begin play
  (bind _asquest_character (Utilities|Casting|CastToQuestCharacter (Pawn|GetControlledPawn)))
  (Variables|Default|SetSelectedCharacter _asquest_character)
  (bind _returnvalue (Game|SpawnActorfromClass "/Game/Inventory/Blueprints/BP_Inventory.BP_Inventory_C" (Math|Transform|MakeTransform "0, 0, 0" "0, 0, 0" "1,1,1") "AlwaysSpawn" 0 7 self 7 1.0 true 0))
  (bind _output_get (Variables|Default|SetInventory _returnvalue))
  (bind _output_get_2 (Variables|Default|SetSpellbookWidget (Variables|/Game/UI/MainWidget.MainWidget_C|GetSpellbokWidget (Variables|/Game/Inventory/Blueprints/BP_Inventory.BP_Inventory_C|GetMainWidget _output_get))))
  (Variables|/Game/Spells/Widgets/SpellbookWidget.SpellbookWidget_C|SetOwningController _output_get_2 self)
  (Variables|/Game/Spells/Widgets/SpellbookWidget.SpellbookWidget_C|SetSelectedCharacter (Variables|Default|GetSpellbookWidget) (Variables|Default|GetSelectedCharacter))
  (bind _asbp_game_instance (Utilities|Casting|CastToBP_GameInstance (Game|GetGameInstance)))
  (Class|QuestGameInstanceBase|UpdateGold _asbp_game_instance)
  (bind _returnvalue_2 (Game|SpawnActorfromClass "/Game/Blueprints/BP_Party.BP_Party_C" (Math|Transform|MakeTransform "0, 0, 0" "0, 0, 0" "1,1,1") "AlwaysSpawn" 0 self 0))
  (Variables|Default|SetParty _returnvalue_2)
  (bind _returnvalue_3 (Game|SpawnActorfromClass "/Game/UI/3DMeshCapture/BP_3DMeshCapture.BP_3DMeshCapture_C" (Math|Transform|MakeTransform "5640290.000000,314830.000000,1429450.000000" "0, 0, 0" "1,1,1") "AlwaysSpawn" 0 (Variables|Default|GetSelectedCharacter) 0))
  (Variables|Default|SetEquipmentWindowMesh _returnvalue_3)
  (Default|HideInventory (Variables|Default|GetInventory))
  (Default|UpdateSelectedCharacter (Variables|Default|GetSpellbookWidget))
  (Variables|Default|SetSpellcastingWidget (Variables|/Game/UI/CharactersWidget.CharactersWidget_C|GetSpellCastingWidget (Variables|/Game/UI/MainWidget.MainWidget_C|GetCharactersWidget (Variables|/Game/Inventory/Blueprints/BP_Inventory.BP_Inventory_C|GetMainWidget (Variables|Default|GetInventory)))))
  (Variables|/Game/Spells/Widgets/SpellCastingWidget.SpellCastingWidget_C|SetPlayerController (Variables|Default|GetSpellcastingWidget) self))

(event EventOnTargetSelected
  ;[0 0.01307 1] Inventory functionality
  (Class|AbilitySystemComponent|TargetConfirm (Ability|GetAbilitySystemComponent (Variables|Default|GetSelectedCharacter))))

(event Input|ActionEvents|InputActionCancelTargeting
  (params (Key :type Key%20Structure))
  ;[0 0.01307 1] Inventory functionality
  (:Pressed
    (if (Variables|Default|GetbIsTargeting)
      (Class|AbilitySystemComponent|TargetCancel (Ability|GetAbilitySystemComponent (Variables|Default|GetSelectedCharacter)))
      (Variables|Default|SetbIsTargeting false)
      (Variables|Default|SetbControllerShouldMoveCharacter true))))

(event Input|KeyboardEvents|LeftShift
  (params (Key :type Key%20Structure))
  ;[0 0.01307 1] Inventory functionality
  ;;[1 1 1] Set left shift (for splitting inventory)
  (:Pressed
    (Variables|Default|SetIsShiftDown true))
  (:Released
    (Variables|Default|SetIsShiftDown false)))

(event Input|KeyboardEvents|I
  (params (Key :type Key%20Structure))
  ;[0 0.01307 1] Inventory functionality
  ;;[1 1 1] Show/Hide Inventory
  (:Pressed
    (UI|ToggleInventory)))

(event Input|KeyboardEvents|W
  (params (Key :type Key%20Structure))
  ;[1 1 1] Debugging
  (:Pressed
    (CallFunction|TryActivateAbility "/Game/Abilities/PlayerAndParty/Spells/WizardSpells/GA_Whirlwind_LesserBase.GA_Whirlwind_LesserBase_C")))

(event Input|KeyboardEvents|R
  (params (Key :type Key%20Structure))
  ;[1 1 1] Debugging
  (:Pressed
    (Default|Rest (Variables|Default|GetParty))))

(event Input|KeyboardEvents|X
  (params (Key :type Key%20Structure))
  ;[1 1 1] Debugging
  (:Pressed
    (CallFunction|TryActivateAbility "/Game/Abilities/PlayerAndParty/Spells/WizardSpells/GA_ErwinsMagicArrowOFDOOM.GA_ErwinsMagicArrowOFDOOM_C")))

(event Input|KeyboardEvents|S
  (params (Key :type Key%20Structure))
  ;[1 1 1] Debugging
  (:Pressed
    (UI|ToggleSpellbookScreen)))

(event Input|KeyboardEvents|H
  (params (Key :type Key%20Structure))
  ;[1 1 1] Debugging
  (:Pressed
    (CallFunction|TryActivateAbility "/Game/Abilities/PlayerAndParty/Spells/PriestSpells/GA_LightHealingSpell.GA_LightHealingSpell_C")))

(event Input|KeyboardEvents|C
  (params (Key :type Key%20Structure))
  (bind _inventory (Variables|Default|GetInventory))
  (bind _mainwidget (Variables|/Game/Inventory/Blueprints/BP_Inventory.BP_Inventory_C|GetMainWidget _inventory))
  (bind _craftingmenuwidget (Variables|/Game/UI/MainWidget.MainWidget_C|GetCraftingMenuWidget _mainwidget))
  ;[1 1 1] Debugging
  ;;[0.001565 0 0.5052] Crafting
  (:Pressed
    (Widget|SetVisibility _craftingmenuwidget (select (Widget|IsVisible _craftingmenuwidget) "Hidden" "Visible"))))

(event Input|KeyboardEvents|SpaceBar
  (params (Key :type Key%20Structure))
  ;[1 1 1] Debugging
  ;;[0.001565 0 0.5052] Pause
  (:Pressed
    (CallFunction|TogglePauseGame)))

(event Input|KeyboardEvents|7
  (params (Key :type Key%20Structure))
  (bind _party (Variables|Default|GetParty))
  ;[1 1 1] Debugging
  ;;[0.001565 0 0.5052] Add player to party
  (:Pressed
    (if (< (Variables|/Game/Blueprints/BP_Party.BP_Party_C|GetCurrentPartySize _party) (Variables|/Game/Blueprints/BP_Party.BP_Party_C|GetMaxPartySize _party))
      (bind _returnvalue (Game|SpawnActorfromClass "/Game/Blueprints/BP_CharacterBase.BP_CharacterBase_C" (Math|Conversions|ToTransform(Vector) (+ (Transformation|GetActorLocation (Game|GetPlayerCharacter 0)) "200.000000, 0, 0")) "AdjustIfPossibleButAlwaysSpawn" 0 "DefaultCharacterName" (Variables|Default|GetParty) 0 (Variables|Default|GetInventory) 0))
      (Default|AddPlayertoParty (Variables|Default|GetParty) _returnvalue (Variables|/Game/Blueprints/BP_CharacterBase.BP_CharacterBase_C|GetCharacterName _returnvalue)))))

(event Input|KeyboardEvents|E
  (params (Key :type Key%20Structure))
  ;[1 1 1] Debugging
  ;;[0.001565 0 0.5052] Open/Close Equipment screen
  (:Pressed
    (UI|ToggleEquipmentScreen)))

(event Input|KeyboardEvents|Q
  (params (Key :type Key%20Structure))
  ;[1 1 1] Debugging
  (:Pressed
    (CallFunction|TryActivateAbility "/Game/Abilities/PlayerAndParty/Spells/WizardSpells/GA_Fireball.GA_Fireball_C")))

(fn ConstructionScript)

(fn TryActivateAbility
  (params (AbilityToActivate :type Quest%20Gameplay%20Ability%20Class%20Reference))
  (Abilities|TryActivateAbilitybyClass (Ability|GetAbilitySystemComponent (Variables|Default|GetSelectedCharacter)) AbilityToActivate true)
  (return))

(fn ToggleEquipmentScreen
  (bind _inventory (Variables|Default|GetInventory))
  (bind _mainwidget (Variables|/Game/Inventory/Blueprints/BP_Inventory.BP_Inventory_C|GetMainWidget _inventory))
  (bind _equipmentwindow (Variables|/Game/UI/MainWidget.MainWidget_C|GetEquipmentWindow _mainwidget))
  (bind _returnvalue (Widget|IsVisible _equipmentwindow))
  (Widget|SetVisibility _equipmentwindow (select _returnvalue "Hidden" "SelfHitTestInvisible"))
  (Widget|SetIsEnabled _equipmentwindow _returnvalue)
  (Variables|Default|SetbIsEquipmentWidgetOpen _returnvalue)
  (UI|UpdateEquipmentWidget)
  (if (Variables|Default|GetbIsSpellbookWidgetOpen)
    (UI|ToggleSpellbookScreen))
  (return))

(fn UpdateEquipmentWidget
  ;[1 1 1] Set local variables
  (bind _asbp_character_base (Utilities|Casting|CastToBP_CharacterBase (Variables|Default|GetSelectedCharacter))
    (:then
      (bind _output_get (LocalVariables|SetLocalCharacterReference _asbp_character_base))
      (LocalVariables|SetLocalEquipmentReference (Variables|/Game/Blueprints/BP_CharacterBase.BP_CharacterBase_C|GetEquipment _output_get))
      (LocalVariables|SetLocalEquipmentWidget (Variables|/Game/UI/MainWidget.MainWidget_C|GetEquipmentWindow (Variables|/Game/Inventory/Blueprints/BP_Inventory.BP_Inventory_C|GetMainWidget (Variables|Default|GetInventory))))
      (LocalVariables|SetLocalAttributeSetComponent (Variables|/Script/Quest.QuestCharacterBase|GetAttributeSetComponent (LocalVariables|GetLocalCharacterReference)))
      ;[1 1 1] Update Equipment widget variables and slots
      (Default|UpdateWidget (LocalVariables|GetLocalEquipmentWidget) (Variables|Default|GetInventory))
      ;[1 1 1] Update 3D Mesh for Equipment Widget
      (Default|UpdateMesh (Variables|Default|GetEquipmentWindowMesh) (LocalVariables|GetLocalCharacterReference))
      (return true))
    (:CastFailed
      (return false))))

(fn UpdateSelectedCharacter
  (params (SelectedCharacter :type BP%20Character%20Base%20Object%20Reference))
  (bind _output_get (Variables|Default|SetSelectedCharacter SelectedCharacter))
  (Class|QuestSelectableComponent|ExecuteonSelected (Variables|/Script/Quest.QuestCharacter|GetSelectableComponent _output_get))
  (UI|UpdateEquipmentWidget)
  (Default|UpdateSelectedCharacter (Variables|Default|GetSpellbookWidget))
  (Variables|/Game/Spells/Widgets/SpellCastingWidget.SpellCastingWidget_C|SetSpellbook (Variables|Default|GetSpellcastingWidget) (Variables|/Script/Quest.QuestCharacterBase|GetSpellbook (Variables|Default|GetSelectedCharacter)))
  (return))

(fn CheckifSelectedCharacterCanLevelUp
  (bind _asbp_character_base (Utilities|Casting|CastToBP_CharacterBase (Variables|Default|GetSelectedCharacter)))
  (bind _canlevelup (Default|CanLevelUp _asbp_character_base))
  (if _canlevelup
    (UI|UpdateEquipmentWidget))
  (return _canlevelup))

(fn ToggleSpellbookScreen
  (bind _inventory (Variables|Default|GetInventory))
  (bind _inventory_2 (Variables|Default|GetInventory))
  (bind _inventory_3 (Variables|Default|GetInventory))
  (bind _mainwidget (Variables|/Game/Inventory/Blueprints/BP_Inventory.BP_Inventory_C|GetMainWidget _inventory_2))
  (bind _mainwidget_2 (Variables|/Game/Inventory/Blueprints/BP_Inventory.BP_Inventory_C|GetMainWidget _inventory_3))
  (bind _spellbokwidget (Variables|/Game/UI/MainWidget.MainWidget_C|GetSpellbokWidget _mainwidget))
  (bind _craftingmenuwidget (Variables|/Game/UI/MainWidget.MainWidget_C|GetCraftingMenuWidget _mainwidget_2))
  (bind _returnvalue (Widget|IsVisible _spellbokwidget))
  (Widget|SetVisibility _spellbokwidget (select _returnvalue "Hidden" "SelfHitTestInvisible"))
  (Widget|SetIsEnabled _spellbokwidget _returnvalue)
  (Variables|Default|SetbIsSpellbookWidgetOpen _returnvalue)
  (UI|UpdateSpellbookWidget)
  (if (Variables|Default|GetbIsSpellbookWidgetOpen)
    (if (Variables|Default|GetbIsEquipmentWidgetOpen)
      (UI|ToggleEquipmentScreen))
    (if (Variables|/Game/Inventory/Blueprints/BP_Inventory.BP_Inventory_C|GetIsVisible _inventory)
      (UI|ToggleInventory (Variables|/Game/Inventory/Blueprints/BP_Inventory.BP_Inventory_C|GetOwningController (Variables|Default|GetInventory))))
    (if (Variables|/Game/Inventory/Blueprints/BP_Inventory.BP_Inventory_C|GetIsStorageOpen _inventory)
      (Default|OnStorageClosed (Variables|/Game/Inventory/Blueprints/BP_StorageItems.BP_StorageItems_C|GetChest (Variables|/Game/Inventory/Widgets/StorageWidget.StorageWidget_C|GetStorage (Variables|/Game/UI/MainWidget.MainWidget_C|GetStorageWidget _mainwidget_2)))))
    (if (Widget|IsVisible _craftingmenuwidget)
      (Widget|SetVisibility _craftingmenuwidget "Hidden"))
    (if (Variables|Default|GetIsShopOpen)
      (Default|OnShopClosed (Variables|Default|GetMerchant)))
    (return)
    (else
      (return))))

(fn UpdateSpellbookWidget
  (Default|UpdateSelectedCharacter (Variables|Default|GetSpellbookWidget))
  (return true))

(fn ToggleInventory
  (bind _inventory (Variables|Default|GetInventory))
  (if (Variables|/Game/Inventory/Blueprints/BP_Inventory.BP_Inventory_C|GetIsVisible (Variables|Default|GetInventory))
    (Default|HideInventory _inventory)
    (else
      (Default|ShowInventory _inventory))))

(fn TogglePauseGame
  (if (Variables|Default|GetbIsGamePaused)
    (Variables|Default|SetbIsGamePaused false)
    (Utilities|Time|SetGlobalTimeDilation 1.0)
    (else
      (Variables|Default|SetbIsGamePaused true)
      (Utilities|Time|SetGlobalTimeDilation 0.0)))
  (return))