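; Base gameplay ability for the priest's Mass Harm spells, with activation deferred to its parent class.
; The target filter rebuilds the target data to hold only unique quest characters that are adverse to the casting character.
; During casting, it spawns a generic effect actor at the owner's transform, configured with particle, scale and duration variables.
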(event Ability|EventActivateAbility
  (|CallParentFunction))

(event Ability|EventOnEndAbility
  (params (bWasCancelled :type Boolean))
  (|CallParentFunction bWasCancelled) ; This node is disabled and will not be called.\nDrag off pins to build functionality.
)

(event EventFilterTargets
  (CallFunction|GetAdverseCharacters))

(event EventLaunchEffectstoPlayDuringCasting
  (CallFunction|LaunchCastingEffect))

(fn GetAdverseCharacters
  (for _array_element (Ability|TargetData|GetActorsfromTargetData (Variables|Default|GetTargetData))
    (bind _asquest_character_base (Utilities|Casting|CastToQuestCharacterBase _array_element))
    (if (Class|QuestCharacterBase|IsAdverse _asquest_character_base (Variables|Default|GetCharacter))
      (Utilities|Array|AddUnique (LocalVariables|GetTargetArray) _asquest_character_base)))
  (Variables|Default|SetTargetData (Ability|TargetData|AbilityTargetDatafromActorArray (LocalVariables|GetTargetArray)))
  (return))

(fn LaunchCastingEffect
  (Game|SpawnActorfromClass "/Game/Abilities/PlayerAndParty/Spells/GlobalBaseSpellAbilities/EffectActors/BP_EffectActorBase.BP_EffectActorBase_C" (Transformation|GetActorTransform (Ability|GetOwningActorfromActorInfo)) "AlwaysSpawn" 0 (Variables|Default|GetParticleSystemTemplate) (Variables|Default|GetEffectScale) (Variables|Default|GetEffectDuration) 0)
  (return))