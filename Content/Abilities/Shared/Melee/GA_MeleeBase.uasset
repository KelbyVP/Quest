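; GA_MeleeBase is a shared melee attack gameplay ability that plays an attack animation and damages the target.
; On activation it commits, plays a random montage from AttackMontages and waits for the Skill.melee.dealDamage gameplay event.
; The event's payload target receives GE_MeleeDamage, so the event drives when and whom the attack hits.
; The ability ends when the montage completes, blends out, is interrupted or is cancelled.
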(event Ability|EventActivateAbility
  (bind _attackmontages (Variables|Default|GetAttackMontages))
  ;[1 1 1] Melee Attack - Play attack animation and do damage to Target Character
  (Ability|CommitAbility)
  (|PlayMontageandWaitProxy "None" (Utilities|Array|Get(acopy) _attackmontages (Math|Random|RandomInteger (Utilities|Array|Length _attackmontages))) 1.0 "None" true 1.0
    (:then
      (bind _payload (Ability|Tasks|WaitGameplayEvent "(TagName=\"skill.melee.dealDamage\")" 0)
        (:EventReceived
          (GameplayEffects|ApplyGameplayEffectToTarget (Ability|TargetData|AbilityTargetDatafromActor (.Target (Utilities|Struct|BreakGameplayEventData _payload))) "/Game/Abilities/Shared/Melee/GE_MeleeDamage.GE_MeleeDamage_C" 1 1))))
    (:OnCompleted
      (Ability|EndAbility :!label _label))
    (:OnBlendOut
      (goto _label))
    (:OnInterrupted
      (goto _label))
    (:OnCancelled
      (goto _label))))

(event Ability|EventOnEndAbility
  (params (bWasCancelled :type Boolean)))