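; Fireball spell ability that launches a BP_Fireball projectile from the caster.
; On activation it sets the character's projectile spell montage, then hands off to the parent ability.
; The LaunchEffects event spawns the fireball at the mesh's sword socket with target data, spell level and a GE_SpellDamage spec.
; ApplyDamage is overridden empty because the projectile deals the damage itself.
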(event Ability|EventActivateAbility
  (bind _characterbase (CallFunction|GetCharacterandControllerInfo))
  (Variables|Default|SetAnimMontageToPlay (Variables|/Game/Blueprints/BP_CharacterBase.BP_CharacterBase_C|GetSpellMontage_Projectile _characterbase))
  (|CallParentFunction))

(event Ability|EventOnEndAbility
  (params (bWasCancelled :type Boolean))
  (|CallParentFunction bWasCancelled) ; This node is disabled and will not be called.\nDrag off pins to build functionality.
)

(event EventApplyDamage
  (params (TargetData :type Gameplay%20Ability%20Target%20Data%20Handle%20Structure%20%28by%20ref%29))
  ;[1 1 1] Override parent's Apply Damage function because damage is done by BP_Fireball
)

(event EventLaunchEffects
  (CallFunction|LaunchFireball))

(fn LaunchFireball
  (Game|SpawnActorfromClass "/Game/Abilities/Shared/WizardSpells/BP_Fireball.BP_Fireball_C" (Transformation|GetSocketTransform (Variables|/Script/Engine.Character|GetMesh (Variables|Default|GetCharacter)) "swordSocket" "RTS_World") "AlwaysSpawn" (Variables|Default|GetCharacter) (Variables|Default|GetTargetLocation) (Variables|Default|GetSpellLevel) (Ability|MakeOutgoingGameplayEffectSpec "/Game/Abilities/Shared/GE_SpellDamage.GE_SpellDamage_C" (Math|Conversions|ToFloat(Integer) (Variables|Default|GetSpellLevel))) (Variables|Default|GetTargetData) 0)
  (return))