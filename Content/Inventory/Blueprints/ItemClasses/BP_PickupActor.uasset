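; BP_PickupActor is a world item pickup that gives an item and amount to the player character on touch.
; Overlapping its sphere casts to BP_PlayerCharacter and, if the Inventory is valid, calls AddItem with ItemToAdd and Amount.
; On success, any leftover count becomes the new Amount so partial pickups stay in the world; otherwise the actor destroys itself.
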(event OnComponentBeginOverlap(Sphere)
  (params (OverlappedComponent :type Primitive%20Component%20Object%20Reference) (OtherActor :type Actor%20Object%20Reference) (OtherComp :type Primitive%20Component%20Object%20Reference) (OtherBodyIndex :type Integer) (bFromSweep :type Boolean) (SweepResult :type Hit%20Result%20Structure%20%28by%20ref%29))
  (bind _asbp_player_character (Utilities|Casting|CastToBP_PlayerCharacter OtherActor))
  (Utilities|IsValid (Variables|/Game/Blueprints/BP_PlayerCharacter.BP_PlayerCharacter_C|GetInventory _asbp_player_character)
    (:Is%20Valid
      (bind (_issuccessful _numbernotadded) (Default|AddItem (Variables|/Game/Blueprints/BP_PlayerCharacter.BP_PlayerCharacter_C|GetInventory _asbp_player_character) (Variables|Default|GetItemToAdd) (Variables|Default|GetAmount)))
      (if _issuccessful
        (if (> _numbernotadded 0)
          (Variables|Default|SetAmount _numbernotadded)
          (else
            (Actor|DestroyActor)))))))

(event EventBeginPlay)

(event Collision|EventActorBeginOverlap
  (params (OtherActor :type Actor%20Object%20Reference)))

(event EventTick
  (params (DeltaSeconds :type Float%20%28single-precision%29)))

(fn ConstructionScript)