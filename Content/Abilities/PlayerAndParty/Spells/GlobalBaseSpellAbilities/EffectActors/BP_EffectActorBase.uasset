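; BP_EffectActorBase is a base actor for timed particle effects, filed under global spell abilities for the player and party.
; On BeginPlay it applies its particle template and scale to the FX component, then activates it.
; After the configured duration it deactivates the effect and waits briefly before destroying itself.
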(event EventBeginPlay
  ;[0 0.07082 1] Set the particle system we'll use
  (Effects|Components|ParticleSystem|SetTemplate (Variables|Default|GetFX) (Variables|Default|GetParticleSystemTemplate))
  ;[1 1 1] Set scale
  (Transformation|SetWorldScale3D (Variables|Default|GetFX) (Variables|Default|GetScale))
  ;[0 0.07082 1] Activate particle effect
  (Components|Activation|Activate (Variables|Default|GetFX) false)
  ;[1 1 1] Set duration
  (Utilities|FlowControl|Delay (Variables|Default|GetDuration))
  ;[1 1 1] Deactivate FX
  (Components|Activation|Deactivate (Variables|Components|GetFX))
  (Utilities|FlowControl|Delay 2.0)
  ;[1 1 1] Destroy actor
  (Actor|DestroyActor))

(fn ConstructionScript)