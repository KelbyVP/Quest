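; Base gameplay ability for ground-targeted spells that spawn an effect actor at a player-confirmed location.
; Activation waits on a ground-select target actor with decal and radius, then turns the character toward the point and plays a montage.
; A gameplay event during the montage commits the ability and spawns the projectile class there, passing the effect spec and target data.
; Children can override OnProjectileLaunched to apply damage from the ability rather than the actor.
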(event Custom|OnProjectileLaunched
  ;[0 0.02624 1] Override this if we want to GA to do damage rather than actor
)

(event Ability|EventActivateAbility
  (|CallParentFunction)
  ;[1 1 1] Get targeting data
  (bind _data (|WaitTargetData :ConfirmationType "UserConfirmed" :Class "/Game/Abilities/PlayerAndParty/BP_GroundTargetSelect.BP_GroundTargetSelect_C" :DecalMaterial (Variables|Default|GetDecalMaterial) :Radius (Variables|Default|GetRadius) :ReticleClass 0)
    (:ValidData
      (Variables|Default|SetTargetData _data)
      (Variables|Default|SetTargetLocation (Class|AbilitySystemBlueprintLibrary|GetTargetDataEndPoint (Variables|Default|GetTargetData) (- (Ability|TargetData|GetDataCountfromTargetData (Variables|Default|GetTargetData)) 1)))
      ;[1 1 1] Turn character toward target
      (Default|TurnTowardTargetLocation (Variables|Default|GetCharacter) (Variables|Default|GetTargetLocation))
      ;[1 1 1] Play spellcasting montage
      (|PlayMontageandWaitProxy "None" (Variables|Default|GetAnimMontageToPlay) 1.0 "None" true 1.0
        (:then
          (Ability|Tasks|WaitGameplayEvent (Variables|Default|GetEventTag) 0
            (:EventReceived
              (Ability|CommitAbility)
              ;[1 1 1] Launch Effects
              (CallFunction|LaunchEffects)
              (CallFunction|OnProjectileLaunched)
              (Ability|EndAbility))))
        (:OnCompleted
          (Ability|EndAbility :!label _label))
        (:OnBlendOut
          (goto _label))
        (:OnInterrupted
          (goto _label))
        (:OnCancelled
          (goto _label))))
    (:Cancelled
      (Ability|EndAbility))))

(event Ability|EventOnEndAbility
  (params (bWasCancelled :type Boolean)))

(fn LaunchEffects
  (Game|SpawnActorfromClass (Variables|Default|GetProjectileClass) (Math|Transform|MakeTransform (Variables|Default|GetTargetLocation) (Math|Rotator|MakeRotator 0.0 0.0 0.0) (Math|Vector|MakeVector 1.0 1.0 1.0)) "AlwaysSpawn" (Variables|Default|GetCharacter) (Variables|Default|GetTargetLocation) (Variables|Default|GetCharacterLevel) (Ability|MakeOutgoingGameplayEffectSpec (Variables|Default|GetGameplayEffectClass) (Math|Conversions|ToFloat(Integer) (Variables|Default|GetCharacterLevel))) (Variables|Default|GetTargetData) 0)
  (return))