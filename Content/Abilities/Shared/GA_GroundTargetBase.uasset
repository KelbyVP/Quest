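; Base Gameplay Ability for ground-targeted area spells, with configurable decal, radius, montage, projectile and damage effect.
; After the player confirms a location, the character turns and plays the montage, whose gameplay event commits the ability and spawns the projectile there.
; An instant second targeting pass gathers actors in range.
; Each receives separately rolled dice damage, with level-scaled bonus dice, as a negative SetByCaller magnitude on the effect spec.
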(event Ability|EventActivateAbility
  (|CallParentFunction)
  (bind _characterbase (CallFunction|GetCharacterandControllerInfo))
  (Variables|Default|SetCharacter _characterbase)
  ;[1 1 1] Get targeting data
  (bind _data (|WaitTargetData :ConfirmationType "UserConfirmed" :Class "/Game/Abilities/PlayerAndParty/BP_GroundTargetSelect.BP_GroundTargetSelect_C" :DecalMaterial (Variables|Default|GetDecalMaterial) :Radius (Variables|Default|GetRadius) :ReticleClass 0)
    (:ValidData
      (Variables|Default|SetTargetData _data)
      (Variables|Default|SetTargetLocation (Class|AbilitySystemBlueprintLibrary|GetTargetDataEndPoint (Variables|Default|GetTargetData) (- (Ability|TargetData|GetDataCountfromTargetData (Variables|Default|GetTargetData)) 1)))
      ;[1 1 1] Turn character toward target
      (Default|TurnTowardTargetLocation (Variables|Default|GetCharacter) (Variables|Default|GetTargetLocation))
      ;[1 1 1] Play spellcasting montage
      (|PlayMontageandWaitProxy "None" (Variables|Default|GetAnimMontageToPlay) 1.0 "None" true 1.0
        (:then
          (Ability|Tasks|WaitGameplayEvent (Variables|Default|GetEventTag) 0
            (:EventReceived
              (Ability|CommitAbility)
              ;[1 1 1] Launch Effects
              (CallFunction|LaunchEffects)
              ;[1 1 1] Damage targets in range
              (bind _data_2 (|WaitTargetData :ConfirmationType "Instant" :Class "/Script/Quest.QuestGATargetActorsInRange" :TargetLocation (Variables|Default|GetTargetLocation) :TargetRadius (Variables|Default|GetRadius))
                (:ValidData
                  (bind _output_get (Variables|Default|SetTargetData _data_2))
                  (CallFunction|ApplyDamage _output_get)
                  (Ability|EndAbility))))))
        (:OnCompleted
          (Ability|EndAbility :!label _label))
        (:OnBlendOut
          (goto _label))
        (:OnInterrupted
          (goto _label))
        (:OnCancelled
          (goto _label))))
    (:Cancelled
      (Ability|EndAbility))))

(event Ability|EventOnEndAbility
  (params (bWasCancelled :type Boolean)))

(fn LaunchEffects
  (Game|SpawnActorfromClass (Variables|Default|GetProjectileClass) (Math|Transform|MakeTransform (Variables|Default|GetTargetLocation) "0, 0, 0" "1,1,1") "AlwaysSpawn" (Variables|Default|GetCharacter) 0)
  (return))

(fn CalculateDamage
  (for _index (range 1 (Variables|Damage|GetNumberOfDamageRolls))
    ;[1 1 1] Set base damage
    (LocalVariables|SetLocalDamage (+ (LocalVariables|GetLocalDamage) (Math|Random|RandomIntegerinRange 1 (Variables|Damage|GetDieSize)))))
  (for _index_2 (range (Variables|Damage|GetSlotLevelForBonusDamage) (Variables|Default|GetCharacterLevel))
    (LocalVariables|SetLocalDamage (+ (LocalVariables|GetLocalDamage) (Math|Random|RandomIntegerinRange 1 (Variables|Damage|GetDieSizeForBonusDamage)))))
  (return (LocalVariables|GetLocalDamage)))

(fn ApplyDamage
  (params (TargetData :type Gameplay%20Ability%20Target%20Data%20Handle%20Structure%20%28by%20ref%29))
  (for _array_element (Ability|TargetData|GetActorsfromTargetData TargetData)
    (bind _damage (CallFunction|CalculateDamage))
    (bind _returnvalue (Ability|GameplayEffect|AssignTagSetbyCallerMagnitude (Ability|MakeOutgoingGameplayEffectSpec (Variables|Default|GetDamageEffect) (Math|Conversions|ToFloat(Integer) (Variables|Default|GetCharacterLevel))) "(TagName=\"spell.Damage\")" (* -1 (Math|Conversions|ToFloat(Integer) _damage))))
    (GameplayEffects|ApplyGameplayEffectSpecToTarget _returnvalue (Ability|TargetData|AbilityTargetDatafromActor _array_element)))
  (return))