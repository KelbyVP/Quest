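; Base merchant character that runs a shop with stock and buy-back.
; Interacting registers it with the game instance and player controller, opens the shop widget and enables inventory Sell All, gated by a DoOnce until closing.
; Obtained items stack by type into stock and enter a capped buy-back list that drops the oldest entry.
; Buy-back charges gold, refunds whatever the inventory cannot hold, then updates both lists and the widget.
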(event Custom|OnShopClosed
  (bind _self self)
  ;[0 0.2708 0.03765] On Shop Closed
  (Default|SetSellAllButton (Variables|/Game/Blueprints/BP_PlayerController.BP_PlayerController_C|GetInventory (Variables|Default|GetPlayerController)) false)
  (Variables|/Game/Blueprints/BP_PlayerController.BP_PlayerController_C|SetIsShopOpen (Variables|Default|GetPlayerController) false)
  (if (Variables|/Game/Inventory/Blueprints/BP_Inventory.BP_Inventory_C|GetIsVisible (Variables|/Game/Blueprints/BP_PlayerController.BP_PlayerController_C|GetInventory (Variables|Default|GetPlayerController)))
    (Default|HideInventory (Variables|/Game/Blueprints/BP_PlayerController.BP_PlayerController_C|GetInventory (Variables|Default|GetPlayerController)))
    (Default|ShowInventory (Variables|/Game/Blueprints/BP_PlayerController.BP_PlayerController_C|GetInventory (Variables|Default|GetPlayerController)))
    (Utilities|IsValid (Variables|Default|GetShopWidget)
      (:Is%20Valid
        (Widget|RemovefromParent (Variables|Default|GetShopWidget) :!label _label))
      (:Is%20Not%20Valid
        _))
    (else
      (goto _label)))
  (Variables|Default|SetShopWidget 0)
  ;[0 0.2708 0.03765] OnInteract
  (Utilities|FlowControl|DoOnce false) ; enters at Reset
)

(event Custom|OnObtainItems
  (params (ObtainedItems :type S%20Inventory%20Slot%20Structure))
  ;[0 0.2708 0.03765] On Obtain Items
  (CallFunction|UpdateBuyBackItems ObtainedItems)
  (CallFunction|AddItemstoStore ObtainedItems))

(event Custom|OnRemoveItems
  (params (ItemsToRemove :type S%20Inventory%20Slot%20Structure))
  ;[1 1 1] On Remove Items
  (CallFunction|RemoveItems ItemsToRemove)
  (Default|UpdateBuyBackItems (Variables|Default|GetShopWidget)))

(event EventOnInteract
  (params (PlayerController :type Quest%20Player%20Controller%20Object%20Reference))
  (bind _self self)
  ;[0 0.2708 0.03765] OnInteract
  (Utilities|FlowControl|DoOnce false
    (:Completed
      (bind _asbp_game_instance (Utilities|Casting|CastToBP_GameInstance (Game|GetGameInstance)))
      (Variables|Default|SetGameInstance _asbp_game_instance)
      (bind _asbp_player_controller (Utilities|Casting|CastToBP_PlayerController PlayerController)
        (:then
          (if (Utilities|IsValid _asbp_player_controller)
            (Variables|Default|SetPlayerController _asbp_player_controller)
            (else
              (bind _asbp_player_controller_2 (Utilities|Casting|CastToBP_PlayerController (Game|GetPlayerController 0) :!label _label))
              (Variables|Default|SetPlayerController _asbp_player_controller_2))))
        (:CastFailed
          (goto _label)))
      (Variables|/Game/Blueprints/BP_GameInstance.BP_GameInstance_C|SetMerchant (Variables|Default|GetGameInstance) _self)
      (Variables|/Game/Blueprints/BP_PlayerController.BP_PlayerController_C|SetMerchant (Variables|Default|GetPlayerController) self)
      (bind _returnvalue (UserInterface|CreateWidget "/Game/Inventory/Widgets/ShopWidget.ShopWidget_C" (Variables|Default|GetPlayerController) _self (Variables|Default|GetPlayerController)))
      (bind _output_get (Variables|Default|SetShopWidget _returnvalue))
      (Class|UserWidget|SetPositioninViewport :self _output_get :bRemoveDPIScale false)
      (Class|UserWidget|SetAnchorsinViewport (Variables|Default|GetShopWidget) (Utilities|Struct|MakeAnchors "(X=0.500000,Y=0.500000)" "(X=0.500000,Y=0.500000)"))
      (Class|UserWidget|SetAlignmentinViewport (Variables|Default|GetShopWidget) "(X=0.500000,Y=0.500000)")
      (UserInterface|Viewport|AddtoViewport (Variables|Default|GetShopWidget) 5)
      (Default|HideInventory (Variables|/Game/Blueprints/BP_PlayerController.BP_PlayerController_C|GetInventory (Variables|Default|GetPlayerController)))
      (Default|ShowInventory (Variables|/Game/Blueprints/BP_PlayerController.BP_PlayerController_C|GetInventory (Variables|Default|GetPlayerController)))
      (Default|SetSellAllButton (Variables|/Game/Blueprints/BP_PlayerController.BP_PlayerController_C|GetInventory (Variables|Default|GetPlayerController)) true)
      (Variables|/Game/Blueprints/BP_PlayerController.BP_PlayerController_C|SetIsShopOpen (Variables|Default|GetPlayerController) true))))

(fn ConstructionScript)

(fn SetFireColor
  (Class|Image|SetBrushfromMaterial (Variables|/Game/Inventory/Widgets/ShopWidget.ShopWidget_C|GetFireMaterial (Variables|Default|GetShopWidget)) (Utilities|Select :Index (Variables|Default|GetFireColor) :NewEnumerator0 "/Game/UI/Material/MI_Fire_Red.MI_Fire_Red" :NewEnumerator1 "/Game/UI/Material/MI_Fire_White.MI_Fire_White" :NewEnumerator2 "/Game/UI/Material/MI_Fire_Green.MI_Fire_Green" :NewEnumerator3 "/Game/UI/Material/MI_Fire_Brown.MI_Fire_Brown" :NewEnumerator4 "/Game/UI/Material/MI_Fire_Blue.MI_Fire_Blue"))
  (return))

(fn UpdateBuyBackItems
  (params (AddedItems :type S%20Inventory%20Slot%20Structure))
  (LocalVariables|SetLocalAddedItems AddedItems)
  (if (>= (Utilities|Array|Length (Variables|Default|GetBuyBackItems)) (Variables|Default|GetNumberOfBuyBackSlots))
    (Utilities|Array|RemoveIndex (Variables|Default|GetBuyBackItems)))
  (Utilities|Array|Add (Variables|Default|GetBuyBackItems) (LocalVariables|GetLocalAddedItems))
  (Default|UpdateBuyBackItemWidgets (Variables|Default|GetShopWidget))
  (return))

(fn AddItemstoStore
  (params (S_InventorySlot :type S%20Inventory%20Slot%20Structure%20%28by%20ref%29))
  (LocalVariables|SetLocalitemsToAdd S_InventorySlot)
  (LocalVariables|SetLocalWasAdded false)
  ;[1 1 1] See whether store already has this item type
  (bind (_array_element _array_index) (Utilities|Array|ForEachLoopwithBreak (Variables|Default|GetItemsForSale) :!label _label)
    (:LoopBody
      (if (== (.ItemType (Utilities|Struct|BreakS_InventorySlot _array_element)) (.ItemType (Utilities|Struct|BreakS_InventorySlot (LocalVariables|GetLocalitemsToAdd))))
        (bind _output_get (Variables|Default|SetSlotWithNewItems _array_index))
        (Utilities|Array|SetArrayElem (Variables|Default|GetItemsForSale) _output_get (Utilities|Struct|MakeS_InventorySlot (.ItemType (Utilities|Struct|BreakS_InventorySlot _array_element)) (+ (.Amount (Utilities|Struct|BreakS_InventorySlot _array_element)) (.Amount (Utilities|Struct|BreakS_InventorySlot (LocalVariables|GetLocalitemsToAdd))))))
        (LocalVariables|SetLocalWasAdded true)
        (goto _label Break)))
    (:Completed
      ;[1 1 1] Add items to store
      (if (LocalVariables|GetLocalWasAdded)
        _
        (else
          (bind _returnvalue (Utilities|Array|Add (Variables|Default|GetItemsForSale) (LocalVariables|GetLocalitemsToAdd)))
          (Variables|Default|SetSlotWithNewItems _returnvalue)))
      (Default|UpdateItemList (Variables|Default|GetShopWidget) (Variables|Default|GetSlotWithNewItems) (Variables|Default|GetItemsForSale))
      (return))))

(fn BuyBackItem
  (params (BuyBackItemWidget :type Buy%20Back%20Item%20Widget%20Object%20Reference))
  ;[0.001565 0 0.5052] Bu back item
  ;;[1 1 1] Set local variables
  (bind _output_get (LocalVariables|SetLocalBuyBackItem (Utilities|Struct|MakeS_InventorySlot (Variables|/Game/Inventory/Widgets/BuyBackItemWidget.BuyBackItemWidget_C|GetAssignedItem BuyBackItemWidget) (Variables|/Game/Inventory/Widgets/BuyBackItemWidget.BuyBackItemWidget_C|GetAmountForSale BuyBackItemWidget))))
  (LocalVariables|SetLocalPrice (Math|Float|Truncate (* (.amount _output_get) (Variables|/Script/Quest.QuestItem|GetValue (.itemtype _output_get)))))
  (bind _asbp_game_instance (Utilities|Casting|CastToBP_GameInstance (Game|GetGameInstance))
    (:then
      (bind _output_get_2 (LocalVariables|SetLocalGameInstance _asbp_game_instance))
      ;;[1 1 1] Reduce gold
      (if (>= (Variables|/Script/Quest.QuestGameInstanceBase|GetGold _output_get_2) (LocalVariables|GetLocalPrice))
        (Class|QuestGameInstanceBase|DecreaseGold (LocalVariables|GetLocalGameInstance) (LocalVariables|GetLocalPrice))
        ;;[1 1 1] Add item to inventory
        (bind (_success _numberofitemsnotadded) (Default|AddItem (Variables|/Game/Blueprints/BP_PlayerController.BP_PlayerController_C|GetInventory (Variables|Default|GetPlayerController)) (.itemtype (LocalVariables|GetLocalBuyBackItem)) (.amount (LocalVariables|GetLocalBuyBackItem)) false))
        (LocalVariables|SetLocalNumberNotAdded _numberofitemsnotadded)
        ;;[1 1 1] If not added to inventory, refund gold
        (if _success
          ;;[1 1 1] If only some items added, refund price of those not added
          (if (== (LocalVariables|GetLocalNumberNotAdded) 0)
            (LocalVariables|SetLocalAmountBoughtBack (.amount (LocalVariables|GetLocalBuyBackItem)))
            (else
              (LocalVariables|SetLocalAmountBoughtBack (- (.amount (LocalVariables|GetLocalBuyBackItem)) (LocalVariables|GetLocalNumberNotAdded)))
              (Class|QuestGameInstanceBase|IncreaseGold (LocalVariables|GetLocalGameInstance) (Math|Float|Truncate (* (LocalVariables|GetLocalNumberNotAdded) (Variables|/Script/Quest.QuestItem|GetValue (.itemtype (LocalVariables|GetLocalBuyBackItem))))))))
          ;;[1 1 1] Remove item from BuyBackItems array
          (bind (_array_element _array_index) (Utilities|Array|ForEachLoopwithBreak (Variables|Default|GetBuyBackItems) :!label _label)
            (:LoopBody
              (if (and (== (.itemtype _array_element) (.itemtype (LocalVariables|GetLocalBuyBackItem))) (== (.amount _array_element) (.amount (LocalVariables|GetLocalBuyBackItem))))
                (Utilities|Array|RemoveIndex (Variables|Default|GetBuyBackItems) _array_index)
                (goto _label Break)))
            (:Completed
              ;;[1 1 1] If not all items were added to inventory, put the rest back in the Buy Back Items array
              (if (== (LocalVariables|GetLocalNumberNotAdded) 0)
                _
                (else
                  (Utilities|Array|Add (Variables|Default|GetBuyBackItems) (Utilities|Struct|MakeS_InventorySlot (.itemtype (LocalVariables|GetLocalBuyBackItem)) (LocalVariables|GetLocalNumberNotAdded)))))
              ;;[1 1 1] Update Buy Back Widgets
              (Default|UpdateBuyBackItemWidgets (Variables|Default|GetShopWidget))
              ;;[1 1 1] Remove items from shop
              (CallFunction|OnRemoveItems (Utilities|Struct|MakeS_InventorySlot (.itemtype (LocalVariables|GetLocalBuyBackItem)) (LocalVariables|GetLocalAmountBoughtBack)))
              (return true)))
          (else
            (Class|QuestGameInstanceBase|IncreaseGold (LocalVariables|GetLocalGameInstance) (LocalVariables|GetLocalPrice))
            (return false)))
        (else
          (return false))))
    (:CastFailed
      (return false))))

(fn RemoveItems
  (params (S_InventorySlot :type S%20Inventory%20Slot%20Structure%20%28by%20ref%29))
  (bind (_itemtype _amount) (Utilities|Struct|BreakS_InventorySlot S_InventorySlot))
  ;[1 1 1] Set local variables
  (LocalVariables|SetLocalItemType _itemtype)
  (LocalVariables|SetLocalAmountToRemove _amount)
  ;[1 1 1] Remove items from ItemsForSale array
  (bind (_array_element _array_index) (Utilities|Array|ForEachLoopwithBreak (Variables|Default|GetItemsForSale) :!label _label)
    (:LoopBody
      (if (== (.ItemType (Utilities|Struct|BreakS_InventorySlot _array_element)) (LocalVariables|GetLocalItemType))
        (bind _output_get (LocalVariables|SetLocalSlotWithRemovedItems _array_index))
        (Utilities|Array|SetArrayElem (Variables|Default|GetItemsForSale) _output_get (Utilities|Struct|MakeS_InventorySlot (.ItemType (Utilities|Struct|BreakS_InventorySlot _array_element)) (- (.Amount (Utilities|Struct|BreakS_InventorySlot _array_element)) (LocalVariables|GetLocalAmountToRemove))))
        (Variables|Default|SetWasRemoved true)
        (goto _label Break)))
    (:Completed
      (if (Variables|Default|GetWasRemoved)
        (if (<= (.amount (Utilities|Array|Get(acopy) (Variables|Default|GetItemsForSale) (LocalVariables|GetLocalSlotWithRemovedItems))) 0)
          ;[1 1 1] If there are none left, remove from the widget
          (Default|RemoveItemforSale (Variables|Default|GetShopWidget) (.itemtype (Utilities|Array|Get(acopy) (Variables|Default|GetItemsForSale) (LocalVariables|GetLocalSlotWithRemovedItems))))
          (Utilities|Array|RemoveIndex (Variables|Default|GetItemsForSale) (LocalVariables|GetLocalSlotWithRemovedItems))
          (return)
          (else
            ;[1 1 1] If there are any left, update the widget
            (Default|UpdateItemList (Variables|Default|GetShopWidget) (LocalVariables|GetLocalSlotWithRemovedItems) (Variables|Default|GetItemsForSale))
            (return)))
        (else
          (return))))))