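; Gameplay ability that lets the player click a target actor for an order and passes it to the character's AI Blackboard.
; On activation it waits for user-confirmed target data from a QuestGATargetActorClicked target actor.
; A valid actor is written to the Order_Target key and the ability ends.
; Target data without an actor reports the order as failed to the OrderHandlingComponent before ending.
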(event Ability|EventActivateAbility
  (|CallParentFunction)
  ;[1 1 1] Get targeting data
  (bind _data (|WaitTargetData :ConfirmationType "UserConfirmed" :Class "/Script/Quest.QuestGATargetActorClicked")
    (:ValidData
      (bind _output_get (Variables|Default|SetTargetData _data))
      ;[1 1 1] Verify we clicked on a character
      (if (Ability|TargetData|TargetDataHasActor _output_get)
        ;[1 1 1] Set blackboard value as target selected
        (AI|Components|Blackboard|SetValueasObject (AI|GetBlackboard (Pawn|GetController (Variables|Default|GetCharacter))) (Utilities|String|StringToName "Order_Target") (Utilities|Array|Get(acopy) (Ability|TargetData|GetActorsfromTargetData (Variables|Default|GetTargetData))))
        (Ability|EndAbility)
        (else
          (Class|QuestOrderHandlingComponent|OnOrderEndedCallback (Variables|/Script/Quest.QuestCharacterBase|GetOrderHandlingComponent (Variables|Default|GetCharacter)) "FAILED")
          (Ability|EndAbility))))))

(event Ability|EventOnEndAbility
  (params (bWasCancelled :type Boolean)))