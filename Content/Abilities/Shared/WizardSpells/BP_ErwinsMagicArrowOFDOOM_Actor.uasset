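; Spell actor for Erwin's Magic Arrow of DOOM in the shared wizard spells, positioned relative to its TargetLocation.
; On BeginPlay it moves 200 units from TargetLocation toward the root's forward vector, which is used as a world point rather than a direction.
; It then calls the parent BeginPlay, and adds no tick, overlap or construction logic of its own.
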(event EventBeginPlay
  (Transformation|SetActorLocation (+ (* (Math|Vector|GetUnitDirection(Vector) (Variables|Default|GetTargetLocation) (Math|Vector|GetForwardVector (Variables|Default|GetDefaultSceneRoot))) 200) (Variables|Default|GetTargetLocation)) false false)
  (|CallParentFunction))

(event Collision|EventActorBeginOverlap
  (params (OtherActor :type Actor%20Object%20Reference)))

(event EventTick
  (params (DeltaSeconds :type Float%20%28single-precision%29))
  (|CallParentFunction 0.0))

(fn ConstructionScript
  (|CallParentFunction))