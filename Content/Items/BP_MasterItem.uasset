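; BP_MasterItem is an item actor, apparently the base for usable inventory items.
; On BeginPlay it casts player character 0 to BP_CharacterBase and stores it as CharacterUsingItem.
; Its EventOnUse prints a use message, removes one unit at its Index from the Inventory, and destroys the actor if removal succeeds.
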(event Custom|EventOnUse
  (Development|PrintString (Utilities|String|Append "You used " ""))
  (bind _success (Default|RemoveItematIndex (Variables|OnSpawn|GetInventory) (Variables|OnSpawn|GetIndex) 1))
  (if _success
    (Actor|DestroyActor)))

(event EventBeginPlay
  (bind _asbp_character_base (Utilities|Casting|CastToBP_CharacterBase (Game|GetPlayerCharacter 0)))
  (Variables|Default|SetCharacterUsingItem _asbp_character_base))

(event Collision|EventActorBeginOverlap
  (params (OtherActor :type Actor%20Object%20Reference)))

(event EventTick
  (params (DeltaSeconds :type Float%20%28single-precision%29)))

(fn ConstructionScript)