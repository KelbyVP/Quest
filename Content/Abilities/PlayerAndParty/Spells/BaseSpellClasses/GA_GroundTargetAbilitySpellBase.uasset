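; Base gameplay ability for ground-targeted spells, which spawns an effect actor at the chosen location.
; On activation it caches the target location, runs an empty pre-cast hook, plays the casting montage and waits for a gameplay event.
; That event commits the ability, spawns the actor with a level-scaled effect spec, radius and duration, then calls the overridable OnProjectileLaunched and ends successfully.
; Any montage completion, blend-out, interruption or cancellation calls OnAbortedCast and ends.
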(event Custom|OnProjectileLaunched
  ;[1 1 1] Override this if we want the GA to do damage rather than actor or a GE
)

(event Ability|EventActivateAbility
  (|CallParentFunction)
  (Variables|Default|SetTargetLocation (Variables|Default|GetLocationToTarget))
  (CallFunction|LaunchPreCastingEffects)
  ;[1 1 1] Play spellcasting montage
  (|PlayMontageandWaitProxy "None" (Variables|Default|GetAnimMontageToPlay) 1.0 "None" true 1.0
    (:then
      (Ability|Tasks|WaitGameplayEvent (Variables|Default|GetEventTag) 0
        (:EventReceived
          (Ability|CommitAbility)
          ;[1 1 1] Launch Effects
          (CallFunction|LaunchPostCastingEffects)
          ;[1 1 1] Execute ability
          (CallFunction|OnProjectileLaunched)
          (CallFunction|OnSuccessfulCast)
          (Ability|EndAbility))))
    (:OnCompleted
      (CallFunction|OnAbortedCast :!label _label)
      (Ability|EndAbility))
    (:OnBlendOut
      (goto _label))
    (:OnInterrupted
      (goto _label))
    (:OnCancelled
      (goto _label))))

(event Ability|EventOnEndAbility
  (params (bWasCancelled :type Boolean)))

(fn LaunchPostCastingEffects
  (Game|SpawnActorfromClass (Variables|Default|GetProjectileClass) (Math|Transform|MakeTransform (Variables|Default|GetTargetLocation) (Math|Rotator|MakeRotator 0.0 0.0 0.0) (Math|Vector|MakeVector 1.0 1.0 1.0)) "AlwaysSpawn" (Variables|Default|GetCharacter) (Variables|Default|GetTargetLocation) (Variables|Default|GetCharacterLevel) (Ability|MakeOutgoingGameplayEffectSpec (Variables|Default|GetGameplayEffectClass) (Math|Conversions|ToFloat(Integer) (Variables|Default|GetCharacterLevel))) (Variables|Default|GetTargetData) (Variables|Default|GetRadius) (Variables|Default|GetDuration) 0)
  (return))

(fn LaunchPreCastingEffects)