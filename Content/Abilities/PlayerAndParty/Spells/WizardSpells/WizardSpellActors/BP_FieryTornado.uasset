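; BP_FieryTornado is a wizard spell actor, a tornado variant that can set characters on fire.
; It inherits its base behavior from a parent class and overrides the ChildEffects event to run a burn check.
; The check merges characters within the effect radius with those already captured.
; Each one not already burning makes an Agility saving throw and receives the GE_Burning gameplay effect on failure.
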(event EventBeginPlay
  (|CallParentFunction) ; This node is disabled and will not be called.\nDrag off pins to build functionality.
)

(event Collision|EventActorBeginOverlap
  (params (OtherActor :type Actor%20Object%20Reference))
  (|CallParentFunction OtherActor) ; This node is disabled and will not be called.\nDrag off pins to build functionality.
)

(event EventTick
  (params (DeltaSeconds :type Float%20%28single-precision%29))
  (|CallParentFunction DeltaSeconds) ; This node is disabled and will not be called.\nDrag off pins to build functionality.
)

(event EventOnCharacterinRange
  (params (ObjectInRange :type Object%20Object%20Reference))
  (|CallParentFunction ObjectInRange))

(event EventChildEffects
  (CallFunction|CheckShouldStartBurning))

(fn ConstructionScript
  (|CallParentFunction))

(fn CheckShouldStartBurning
  ;[1 1 1] Identify characters in range and already captured
  (bind _returnvalue (Class|QuestOrderHelperLibrary|GetCharactersinRange self (Variables|Default|GetEffectRadius)))
  (LocalVariables|SetLocalCharactersToCheck _returnvalue)
  (for _array_element (Variables|Default|GetCapturedCharacters)
    (Utilities|Array|AddUnique (LocalVariables|GetLocalCharactersToCheck) _array_element))
  (for _array_element_2 (LocalVariables|GetLocalCharactersToCheck)
    (LocalVariables|SetLocalCharacterToBurn _array_element_2)
    (bind _returnvalue_2 (Class|QuestCharacterBase|DoesCharacterHaveTag (LocalVariables|GetLocalCharacterToBurn) (Utilities|Struct|MakeGameplayTag "(TagName=\"status.burning\")")))
    (if (not _returnvalue_2)
      (bind _returnvalue_3 (Class|QuestAttributeSet|DoesMakeSavingThrow (Variables|/Script/Quest.QuestCharacterBase|GetAttributeSetComponent (LocalVariables|GetLocalCharacterToBurn)) "IT_Agility"))
      (if (not _returnvalue_3)
        (GameplayEffects|ApplyGameplayEffectToSelf :self (Variables|/Script/Quest.QuestCharacterBase|GetAbilitySystemComponent (LocalVariables|GetLocalCharacterToBurn)) :GameplayEffectClass "/Game/Abilities/PlayerAndParty/Spells/WizardSpells/WizardGameplayEffects/GE_Burning.GE_Burning_C"))))
  (return))