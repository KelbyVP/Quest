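; Base actor for a wizard whirlwind spell that damages, stuns and spins characters entering its sphere.
; Overlap applies the ability's effect spec; a failed Strength save spawns a QuestCharacterRotationActor to orbit the victim.
; Looping timers roll escape saves and run ChildEffects, which child classes override alongside CheckOtherSaves.
; After its duration, the effect deactivates, drops remaining captives and destroys itself.
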(event OnComponentBeginOverlap(SphereCollisionComponent)
  (params (OverlappedComponent :type Primitive%20Component%20Object%20Reference) (OtherActor :type Actor%20Object%20Reference) (OtherComp :type Primitive%20Component%20Object%20Reference) (OtherBodyIndex :type Integer) (bFromSweep :type Boolean) (SweepResult :type Hit%20Result%20Structure%20%28by%20ref%29))
  ;[1 1 1] Begin Overlap
  (CallFunction|OnCharacterinRange OtherActor))

(event Custom|OnCharacterDropped
  (params (DroppedCharacter :type Quest%20Character%20Base%20Object%20Reference))
  ;[1 1 1] On Character Dropped (gives the character 5 seconds safety before it can be spun again)
  (Utilities|FlowControl|Delay 5.0)
  (Variables|/Script/Quest.QuestCharacterBase|SetbIsCapturedByRotationActor DroppedCharacter false))

(event EventBeginPlay
  ;[1 1 1] Begin Play
  ;;[0 0.07082 1] Set the particle system we'll use
  (Effects|Components|ParticleSystem|SetTemplate (Variables|Default|Getfx) (Variables|Default|GetParticleSystemTemplate))
  (|CallParentFunction)
  ;;[0 0.07082 1] Activate particle effect
  (Components|Sphere|SetSphereRadius (Variables|Default|GetSphereCollisionComponent) (Variables|Default|GetEffectRadius) false)
  (Components|Activation|Activate (Variables|Default|Getfx) false)
  (bind _returnvalue (Utilities|Time|SetTimerbyFunctionName 0 "CheckSaves" 3.0 true))
  ;;[0 0.07082 1] Override child effects in child class for additional effects
  (Utilities|Time|SetTimerbyFunctionName 0 "ChildEffects" 3.0 true)
  ;;[0 0.07082 1] Set lifespan
  (Utilities|FlowControl|Delay (Variables|Default|GetDuration))
  (Utilities|Time|ClearandInvalidateTimerbyHandle _returnvalue)
  ;;[0 0.07082 1] End whirlwhind
  (Components|Activation|Deactivate (Variables|Default|Getfx))
  (Utilities|FlowControl|Delay 1.0)
  (CallFunction|DropCharacters)
  (Utilities|FlowControl|Delay 2.0)
  ;;[0 0.07082 1] Destroy actor
  (Actor|DestroyActor))

(fn ConstructionScript)

(fn DamageActor
  (params (ActorToDamage :type Actor%20Object%20Reference))
  (bind _asquest_character_base (Utilities|Casting|CastToQuestCharacterBase ActorToDamage)
    (:then
      (Class|QuestFunctionLibrary|ApplyGameplayEffectSpecHandletoTargetDataHandleSpecHandle (Variables|Default|GetEffectSpecHandleFromAbility) (Ability|TargetData|AbilityTargetDatafromActor _asquest_character_base))
      (return))
    (:CastFailed
      (return))))

(fn OnCharacterinRange
  (params (ObjectInRange :type Object%20Object%20Reference))
  (bind _asquest_character_base (Utilities|Casting|CastToQuestCharacterBase ObjectInRange)
    (:then
      (bind _output_get (LocalVariables|SetLocalCharacterInRange _asquest_character_base))
      (if (Variables|/Script/Quest.QuestCharacterBase|GetbIsCapturedByRotationActor _output_get)
        (return)
        (else
          (CallFunction|DamageActor (LocalVariables|GetLocalCharacterInRange))
          (bind _returnvalue (Class|QuestAttributeSet|DoesMakeSavingThrow (Variables|/Script/Quest.QuestCharacterBase|GetAttributeSetComponent (LocalVariables|GetLocalCharacterInRange)) "IT_Strength"))
          (if _returnvalue
            (return)
            (else
              (CallFunction|SpinCharacter (LocalVariables|GetLocalCharacterInRange))
              (return))))))
    (:CastFailed
      (return))))

(fn SpinCharacter
  (params (CharacterInRange :type Quest%20Character%20Base%20Object%20Reference))
  (bind _output_get (LocalVariables|SetLocalCharacter CharacterInRange))
  (Class|QuestCharacterBase|AddGameplayTag _output_get "(TagName=\"status.stunned\")")
  (bind _returnvalue (Game|SpawnActorfromClass "/Script/Quest.QuestCharacterRotationActor" (Math|Transform|MakeTransform "0, 0, 0" "0, 0, 0" "1,1,1") "AlwaysSpawn" 0 (Variables|Default|GetEffectRadius) (Variables|Default|GetMovementSpeedToStartingRotationPosition) (Variables|Default|GetRotationSpeed) (Math|Random|RandomFloatinRange (Variables|Default|GetMinSpinHeight) (Variables|Default|GetMaxSpinHeight)) true (LocalVariables|GetLocalCharacter) self 0))
  (Utilities|Array|AddUnique (Variables|Default|GetRotationActors) _returnvalue)
  (Variables|/Script/Quest.QuestCharacterBase|SetbIsCapturedByRotationActor (LocalVariables|GetLocalCharacter) true)
  (return))

(fn DropCharacters
  (for _array_element (Variables|Default|GetRotationActors)
    (bind _output_get (LocalVariables|SetLocalRotationActor _array_element))
    (bind _asquest_character_base (Utilities|Casting|CastToQuestCharacterBase (Variables|/Script/Quest.QuestCharacterRotationActor|GetCharacterToRotate _output_get)))
    (CallFunction|Escape _asquest_character_base (LocalVariables|GetLocalRotationActor)))
  (return))

(fn CheckSaves
  ;[1 1 1] Loop through rotation actors
  (for _array_element (Variables|Default|GetRotationActors)
    ;[1 1 1] Check save
    (bind _output_get (LocalVariables|SetLocalRotatorToCheck _array_element))
    (bind _asquest_character_base (Utilities|Casting|CastToQuestCharacterBase (Variables|/Script/Quest.QuestCharacterRotationActor|GetCharacterToRotate _output_get)))
    (bind _output_get_2 (LocalVariables|SetLocalCharacterToCheck _asquest_character_base))
    ;;[0 0.07082 1] Override this function in child class for other effects
    (CallFunction|CheckOtherSaves _output_get_2)
    (bind _returnvalue (Class|QuestAttributeSet|DoesMakeSavingThrow (Variables|/Script/Quest.QuestCharacterBase|GetAttributeSetComponent (LocalVariables|GetLocalCharacterToCheck)) (Variables|Default|GetSaveTypeToEscapeSpin)))
    ;[1 1 1] If save made, escape
    (if _returnvalue
      (CallFunction|Escape (LocalVariables|GetLocalCharacterToCheck) (LocalVariables|GetLocalRotatorToCheck))))
  (return))

(fn Escape
  (params (CharacterToEscape :type Quest%20Character%20Base%20Object%20Reference) (RotatorToDestroy :type Quest%20Character%20Rotation%20Actor%20Object%20Reference))
  (Class|QuestCharacterBase|RemoveGameplayTag CharacterToEscape "(TagName=\"status.stunned\")")
  (Utilities|Array|RemoveItem (Variables|Default|GetRotationActors) RotatorToDestroy)
  (Actor|DestroyActor RotatorToDestroy))

(fn CheckOtherSaves
  (params (CharacterToCheck :type Quest%20Character%20Base%20Object%20Reference))
  (return))

(fn ChildEffects
  (return))