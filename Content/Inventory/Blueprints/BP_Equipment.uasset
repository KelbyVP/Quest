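; BP_Equipment tracks equipped items in separate slot arrays for weapons, shields, amulets, rings and quick items, each sized to its maximum on BeginPlay.
; Functions switch on item type to find the first empty slot or set an item at an index, casting all but potions to their item class.
; Potions use quick item slots, and materials have no slot.
; Unequipping clears either a verified index or the first matching entry, keeping array sizes fixed.
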(event EventBeginPlay
  ;[0.001565 0 0.5052] Begin Play
  ;;[1 1 1] Set slots arrays to proper number of elements
  (Utilities|Array|Resize (Variables|Default|GetWeaponSlots) (Variables|Default|GetMaxWeapons))
  (Utilities|Array|Resize (Variables|Default|GetAmuletSlots) (Variables|Default|GetMaxAmulets))
  (Utilities|Array|Resize (Variables|Default|GetRingSlots) (Variables|Default|GetMaxRings))
  (Utilities|Array|Resize (Variables|Default|GetQuickItemSlots) (Variables|Default|GetMaxQuickItems))
  (Utilities|Array|Resize (Variables|Default|GetShieldSlots) (Variables|Default|GetMaxShields)))

(event Collision|EventActorBeginOverlap
  (params (OtherActor :type Actor%20Object%20Reference)))

(event EventTick
  (params (DeltaSeconds :type Float%20%28single-precision%29)))

(fn ConstructionScript)

(fn FindAvailableSlotforItemType
  (params (ItemType :type EItemType%20Enum :default "IT_Potion"))
  (switch Utilities|FlowControl|Switch|SwitchonEItemType ItemType
    (:IT_Potion
      ;[1 1 1] Find slot for Quick Item
      (bind (_array_element _array_index) (Utilities|Array|ForEachLoopwithBreak (Variables|Default|GetQuickItemSlots) :!label _label)
        (:LoopBody
          (Utilities|IsValid _array_element
            (:Is%20Not%20Valid
              (LocalVariables|SetLocalIsSlotFound true)
              (LocalVariables|SetLocalIndexOfFirstAvailableSlotFound _array_index)
              (goto _label Break))))
        (:Completed
          _)))
    (:IT_Weapon
      ;[1 1 1] Find slot for Weapon
      (bind (_array_element_2 _array_index_2) (Utilities|Array|ForEachLoopwithBreak (Variables|Default|GetWeaponSlots) :!label _label_2)
        (:LoopBody
          (Utilities|IsValid _array_element_2
            (:Is%20Not%20Valid
              (LocalVariables|SetLocalIsSlotFound true)
              (bind _output_get (LocalVariables|SetLocalIndexOfFirstAvailableSlotFound _array_index_2))
              (Development|PrintString (Utilities|String|Append "slot found at index " (Utilities|String|ToString(Integer) _output_get)))
              (goto _label_2 Break))))
        (:Completed
          _)))
    (:IT_Ring
      ;[1 1 1] Find slot for Ring
      (bind (_array_element_3 _array_index_3) (Utilities|Array|ForEachLoopwithBreak (Variables|Default|GetRingSlots) :!label _label_3)
        (:LoopBody
          (Utilities|IsValid _array_element_3
            (:Is%20Not%20Valid
              (LocalVariables|SetLocalIsSlotFound true)
              (LocalVariables|SetLocalIndexOfFirstAvailableSlotFound _array_index_3)
              (goto _label_3 Break))))
        (:Completed
          _)))
    (:IT_Material
      (return false 0))
    (:IT_Amulet
      ;[1 1 1] Find slot for Amulet
      (bind (_array_element_4 _array_index_4) (Utilities|Array|ForEachLoopwithBreak (Variables|Default|GetAmuletSlots) :!label _label_4)
        (:LoopBody
          (Utilities|IsValid _array_element_4
            (:Is%20Not%20Valid
              (LocalVariables|SetLocalIsSlotFound true)
              (LocalVariables|SetLocalIndexOfFirstAvailableSlotFound _array_index_4)
              (goto _label_4 Break))))
        (:Completed
          _)))
    (:IT_Shield
      ;[1 1 1] Find slot for Shield
      (bind (_array_element_5 _array_index_5) (Utilities|Array|ForEachLoopwithBreak (Variables|Default|GetShieldSlots) :!label _label_5)
        (:LoopBody
          (Utilities|IsValid _array_element_5
            (:Is%20Not%20Valid
              (LocalVariables|SetLocalIsSlotFound true)
              (LocalVariables|SetLocalIndexOfFirstAvailableSlotFound _array_index_5)
              (goto _label_5 Break))))
        (:Completed
          _))))
  (return (LocalVariables|GetLocalIsSlotFound) (LocalVariables|GetLocalIndexOfFirstAvailableSlotFound)))

(fn EquipItematIndex
  (params (Index :type Integer) (ItemTypeEnum :type EItemType%20Enum :default "IT_Potion") (ItemToEquip :type Quest%20Item%20Object%20Reference))
  ;[1 1 1] Set local variables
  (LocalVariables|SetLocalIndexToEquip Index)
  (LocalVariables|SetLocalItemTypeEnum ItemTypeEnum)
  (LocalVariables|SetLocalItemToEquip ItemToEquip)
  (switch Utilities|FlowControl|Switch|SwitchonEItemType (LocalVariables|GetLocalItemTypeEnum)
    (:IT_Potion
      ;[1 1 1] Set quick item in slot
      (Utilities|Array|SetArrayElem (Variables|Default|GetQuickItemSlots) (LocalVariables|GetLocalIndexToEquip) (LocalVariables|GetLocalItemToEquip)))
    (:IT_Weapon
      ;[1 1 1] Set weapon in slot
      (bind _asquest_weapon_item (Utilities|Casting|CastToQuestWeaponItem (LocalVariables|GetLocalItemToEquip)))
      (Utilities|Array|SetArrayElem (Variables|Default|GetWeaponSlots) (LocalVariables|GetLocalIndexToEquip) _asquest_weapon_item))
    (:IT_Ring
      ;[1 1 1] Set ring in slot
      (bind _asquest_ring_item (Utilities|Casting|CastToQuestRingItem (LocalVariables|GetLocalItemToEquip)))
      (Utilities|Array|SetArrayElem (Variables|Default|GetRingSlots) (LocalVariables|GetLocalIndexToEquip) _asquest_ring_item))
    (:IT_Amulet
      ;[1 1 1] Set amulet in slot
      (bind _asquest_amulet_item (Utilities|Casting|CastToQuestAmuletItem (LocalVariables|GetLocalItemToEquip)))
      (Utilities|Array|SetArrayElem (Variables|Default|GetAmuletSlots) (LocalVariables|GetLocalIndexToEquip) _asquest_amulet_item))
    (:IT_Shield
      ;[1 1 1] Set shield in slot
      (bind _asquest_shield_item (Utilities|Casting|CastToQuestShieldItem (LocalVariables|GetLocalItemToEquip)))
      (Utilities|Array|SetArrayElem (Variables|Default|GetShieldSlots) (LocalVariables|GetLocalIndexToEquip) _asquest_shield_item)))
  (return))

(fn UnequipItem
  (params (ItemToUnequip :type Quest%20Item%20Object%20Reference) (ShouldUnequipSpecificIndex :type Boolean) (IndexToUnequip :type Integer))
  ;[1 1 1] Set local variables
  (LocalVariables|SetLocalItemToUnequip ItemToUnequip)
  (LocalVariables|SetLocalShouldUnequipSpecificIndex ShouldUnequipSpecificIndex)
  (LocalVariables|SetLocalIndexToUnequip IndexToUnequip)
  (if (LocalVariables|GetLocalShouldUnequipSpecificIndex)
    ;[1 1 1] Decide which array has the item
    (bind _isremoved (CallFunction|RemoveItematIndex (Utilities|Select :Index (Variables|/Script/Quest.QuestItem|GetItemTypeEnum (LocalVariables|GetLocalItemToUnequip)) :IT_Potion (Variables|Default|GetQuickItemSlots) :IT_Weapon (Variables|Default|GetWeaponSlots) :IT_Ring (Variables|Default|GetRingSlots) :IT_Material 0 :IT_Amulet (Variables|Default|GetAmuletSlots) :IT_Shield (Variables|Default|GetShieldSlots)) (LocalVariables|GetLocalIndexToUnequip) (LocalVariables|GetLocalItemToUnequip)))
    (return _isremoved)
    (else
      ;[1 1 1] Find the item and remove it from the array
      (bind (_array_element _array_index) (Utilities|Array|ForEachLoopwithBreak (Utilities|Select :Index (Variables|/Script/Quest.QuestItem|GetItemTypeEnum (LocalVariables|GetLocalItemToUnequip)) :IT_Potion (Variables|Default|GetQuickItemSlots) :IT_Weapon (Variables|Default|GetWeaponSlots) :IT_Ring (Variables|Default|GetRingSlots) :IT_Material 0 :IT_Amulet (Variables|Default|GetAmuletSlots) :IT_Shield (Variables|Default|GetShieldSlots)) :!label _label)
        (:LoopBody
          (if (== _array_element (LocalVariables|GetLocalItemToUnequip))
            (Utilities|Array|SetArrayElem (Utilities|Select :Index (Variables|/Script/Quest.QuestItem|GetItemTypeEnum (LocalVariables|GetLocalItemToUnequip)) :IT_Potion (Variables|Default|GetQuickItemSlots) :IT_Weapon (Variables|Default|GetWeaponSlots) :IT_Ring (Variables|Default|GetRingSlots) :IT_Material 0 :IT_Amulet (Variables|Default|GetAmuletSlots) :IT_Shield (Variables|Default|GetShieldSlots)) _array_index 0)
            (LocalVariables|SetLocalIsRemoved true)
            (goto _label Break)))
        (:Completed
          (Development|PrintString (Utilities|String|Append "item removed? " (Utilities|String|ToString(Boolean) (LocalVariables|GetLocalIsRemoved))))
          (return (LocalVariables|GetLocalIsRemoved)))))))

(fn RemoveItematIndex
  (params (ArrayContainingItem :type Array%20of%20Quest%20Item%20Object%20References) (Index :type Integer) (ItemToRemove :type Quest%20Item%20Object%20Reference))
  (if (== (Utilities|Array|Get(acopy) ArrayContainingItem Index) ItemToRemove)
    (Utilities|Array|SetArrayElem ArrayContainingItem Index 0)
    (return true)
    (else
      (return false))))