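; Priest gameplay ability for the Mass Light Healing spell, whose own graph only narrows the spell's targets to allies.
; FilterTargets runs GetAlliedCharacters, which takes actors from the target data and collects unique QuestCharacterBase characters allied to Character.
; It then rebuilds TargetData from that array; activation, ending and healing are not implemented in these graphs.
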(event Ability|EventActivateAbility
  (|CallParentFunction) ; This node is disabled and will not be called.\nDrag off pins to build functionality.
)

(event Ability|EventOnEndAbility
  (params (bWasCancelled :type Boolean))
  (|CallParentFunction bWasCancelled) ; This node is disabled and will not be called.\nDrag off pins to build functionality.
)

(event EventFilterTargets
  (CallFunction|GetAlliedCharacters))

(fn GetAlliedCharacters
  (for _array_element (Ability|TargetData|GetActorsfromTargetData (Variables|Default|GetTargetData))
    (bind _asquest_character_base (Utilities|Casting|CastToQuestCharacterBase _array_element))
    (if (Class|QuestCharacterBase|IsAllied _asquest_character_base (Variables|Default|GetCharacter))
      (Utilities|Array|AddUnique (LocalVariables|GetTargetArray) _asquest_character_base)))
  (Variables|Default|SetTargetData (Ability|TargetData|AbilityTargetDatafromActorArray (LocalVariables|GetTargetArray)))
  (return))