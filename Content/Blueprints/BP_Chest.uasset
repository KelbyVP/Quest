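; BP_Chest is an interactable container that opens a storage window alongside the player's inventory.
; On interact, a DoOnce gate lazily spawns a BP_Storage actor with the chest's slot layout, generates its slot widgets, then shows it and refreshes the inventory.
; Closing storage hides it, refreshes any visible inventory and resets the gate.
; The overlap event only casts to QuestCharacter, with no further effect.
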(event Custom|OnStorageClosed
  ;[1 1 1] On Storage Closed
  (Default|HideStorage (Variables|Default|GetStorageActor))
  (if (Variables|/Game/Inventory/Blueprints/BP_Inventory.BP_Inventory_C|GetIsVisible (Variables|/Game/Blueprints/BP_PlayerController.BP_PlayerController_C|GetInventory (Variables|Default|GetPlayerController)))
    (Default|HideInventory (Variables|/Game/Blueprints/BP_PlayerController.BP_PlayerController_C|GetInventory (Variables|Default|GetPlayerController)))
    (Default|ShowInventory (Variables|/Game/Blueprints/BP_PlayerController.BP_PlayerController_C|GetInventory (Variables|Default|GetPlayerController)))
    ;[1 1 1] On Interact
    (Utilities|FlowControl|DoOnce false) ; enters at Reset
    (else
      (Utilities|FlowControl|DoOnce false) ; enters at Reset
    )))

(event EventBeginPlay)

(event Collision|EventActorBeginOverlap
  (params (OtherActor :type Actor%20Object%20Reference))
  (bind _asquest_character (Utilities|Casting|CastToQuestCharacter OtherActor)))

(event EventTick
  (params (DeltaSeconds :type Float%20%28single-precision%29)))

(event EventOnInteract
  (params (PlayerController :type Quest%20Player%20Controller%20Object%20Reference))
  ;[1 1 1] On Interact
  (Utilities|FlowControl|DoOnce false
    (:Completed
      (bind _asbp_player_controller (Utilities|Casting|CastToBP_PlayerController PlayerController))
      (Variables|Default|SetPlayerController _asbp_player_controller)
      (Utilities|IsValid (Variables|Default|GetStorageActor)
        (:Is%20Valid
          _)
        (:Is%20Not%20Valid
          (bind _returnvalue (Game|SpawnActorfromClass "/Game/Inventory/Blueprints/BP_Storage.BP_Storage_C" (Math|Transform|MakeTransform "0, 0, 0" "0, 0, 0" "1,1,1") "AlwaysSpawn" 0 (Variables|Default|GetAmountOfSlots) (Variables|Default|GetPlayerController) (Variables|Default|GetSlotsPerRow) self 0))
          (bind _output_get (Variables|Default|SetStorageActor _returnvalue))
          (Default|GenerateSlotWidgets (Variables|/Game/Inventory/Blueprints/BP_Storage.BP_Storage_C|GetStorageWidget (Variables|Default|GetStorageActor)) _output_get)))
      (Default|ShowStorage (Variables|Default|GetStorageActor))
      (Default|HideInventory (Variables|/Game/Blueprints/BP_PlayerController.BP_PlayerController_C|GetInventory (Variables|Default|GetPlayerController)))
      (Default|ShowInventory (Variables|/Game/Blueprints/BP_PlayerController.BP_PlayerController_C|GetInventory (Variables|Default|GetPlayerController))))))

(fn ConstructionScript)