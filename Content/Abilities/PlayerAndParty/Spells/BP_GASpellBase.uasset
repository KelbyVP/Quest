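; BP_GASpellBase is a base gameplay ability for character spells, with memorized spells used up only on a successful cast.
; On activation it caches the owning BP_CharacterBase, its level from the attribute set and its projectile spell montage.
; Success and abort events both report the spell class to the character through OnSpellFinished, flagging whether to remove it from memorized spells.
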(event Custom|OnSuccessfulCast
  ;[1 1 1] On successful cast
  (Default|OnSpellFinished (Variables|Default|GetCharacter) (Utilities|GetClass self) true))

(event Custom|OnAbortedCast
  ;[1 1 1] On aborted cast
  (Default|OnSpellFinished (Variables|Default|GetCharacter) (Utilities|GetClass self) false))

(event Ability|EventActivateAbility
  ;[1 1 1] Activate ability
  (CallFunction|SetCharacterVariables))

(fn GetCharacterandControllerInfo
  (bind _asbp_character_base (Utilities|Casting|CastToBP_CharacterBase (Ability|GetOwningActorfromActorInfo))
    (:then
      (bind _asbp_player_controller (Utilities|Casting|CastToBP_PlayerController (Game|GetPlayerController 0)))
      (return _asbp_character_base _asbp_player_controller))
    (:CastFailed
      (return 0 0))))

(fn SetCharacterVariables
  (bind _characterbase (CallFunction|GetCharacterandControllerInfo))
  (Variables|Default|SetCharacter _characterbase)
  (bind _output_get (Variables|Default|SetCharacterLevel (Math|Float|Truncate (.currentvalue (Variables|/Script/Quest.QuestAttributeSet|GetLevel (Variables|/Script/Quest.QuestCharacterBase|GetAttributeSetComponent (Variables|Default|GetCharacter)))))))
  (Variables|Default|SetAnimMontageToPlay (Variables|/Game/Blueprints/BP_CharacterBase.BP_CharacterBase_C|GetSpellMontage_Projectile (Variables|Default|GetCharacter)))
  (return _output_get))