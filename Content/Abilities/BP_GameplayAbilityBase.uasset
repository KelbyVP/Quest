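; Base Gameplay Ability Blueprint that sets a spell level from the owning character's Level attribute on activation.
; ActivateAbility calls SetLevel, which truncates the base Level value from the character's AttributeSetComponent into SpellLevel.
; GetCharacterAndControllerInfo is the shared helper that casts the owning actor to BP_CharacterBase and its controller to BP_PlayerController, returning both.
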(event Ability|EventActivateAbility
  (CallFunction|SetLevel))

(event Ability|EventOnEndAbility
  (params (bWasCancelled :type Boolean)))

(fn GetCharacterandControllerInfo
  (bind _asbp_character_base (Utilities|Casting|CastToBP_CharacterBase (Ability|GetOwningActorfromActorInfo))
    (:then
      (bind _asbp_player_controller (Utilities|Casting|CastToBP_PlayerController (Pawn|GetController _asbp_character_base)))
      (return _asbp_character_base _asbp_player_controller))
    (:CastFailed
      (return 0 0))))

(fn SetLevel
  (bind _characterbase (CallFunction|GetCharacterandControllerInfo))
  (bind _output_get (Variables|Default|SetSpellLevel (Math|Float|Truncate (.basevalue (Variables|/Script/Quest.QuestAttributeSet|GetLevel (Variables|/Script/Quest.QuestCharacterBase|GetAttributeSetComponent _characterbase))))))
  (return _output_get))