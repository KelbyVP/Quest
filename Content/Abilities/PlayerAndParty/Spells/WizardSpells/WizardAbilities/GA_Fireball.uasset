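; GA_Fireball is the wizard's fireball spell ability, built on a parent casting ability class.
; After casting, it spawns BP_Fireball_Actor 750 units above the caster's sword socket, passing target location, level, radius, target data and a GE_SpellDamage spec.
; It overrides the parent's ApplyDamage to do nothing, because the fireball actor deals the damage itself.
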(event Custom|ApplyDamage
  (params (TargetData :type Gameplay%20Ability%20Target%20Data%20Handle%20Structure%20%28by%20ref%29))
  ;[1 1 1] Override parent's Apply Damage function because damage is done by BP_Fireball
)

(event Ability|EventActivateAbility
  (|CallParentFunction))

(event Ability|EventOnEndAbility
  (params (bWasCancelled :type Boolean))
  (|CallParentFunction bWasCancelled) ; This node is disabled and will not be called.\nDrag off pins to build functionality.
)

(event EventLaunchPostCastingEffects
  (CallFunction|LaunchFireball))

(fn LaunchFireball
  (bind _character (Variables|Default|GetCharacter))
  (bind _mesh (Variables|/Script/Engine.Character|GetMesh _character))
  (bind _returnvalue (Transformation|GetSocketTransform _mesh "swordSocket" "RTS_World"))
  (Game|SpawnActorfromClass "/Game/Abilities/PlayerAndParty/Spells/WizardSpells/WizardSpellActors/BP_Fireball_Actor.BP_Fireball_Actor_C" (Math|Transform|MakeTransform (Math|Vector|MakeVector (.x (.location _returnvalue)) (.y (.location _returnvalue)) (+ (.z (.location _returnvalue)) 7.5e+02)) (.rotation _returnvalue) (.scale _returnvalue)) "AlwaysSpawn" (Variables|Default|GetCharacter) (Variables|Default|GetLocationToTarget) (Variables|Default|GetCharacterLevel) (Ability|MakeOutgoingGameplayEffectSpec "/Game/Abilities/Shared/GE_SpellDamage.GE_SpellDamage_C" (Math|Conversions|ToFloat(Integer) (Variables|Default|GetCharacterLevel))) (Variables|Default|GetTargetData) (Variables|Default|GetRadius) 0)
  (return))